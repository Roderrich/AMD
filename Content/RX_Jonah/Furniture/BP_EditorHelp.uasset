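; BP_EditorHelp is a spinning helper actor that lasts only as long as the actor it is meant to draw attention to, ActorNeedToBeNoticed.
; From BeginPlay, a looping short-interval timer checks that reference and, while valid, restarts a timeline that lerps the helper's current rotation toward an added yaw step.
; Once the reference is invalid, it clears its flag and timer, then destroys itself.
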(event Custom|StartCheckIsNoticedItemExisted
  (bind _returnvalue (Utilities|Time|SetTimerbyEvent (delegate Custom|IsItemExisted) 0.2 true))
  (Variables|Default|SetCheckItemExictingTimer _returnvalue))

(event Custom|IsItemExisted
  (bind _returnvalue (Transformation|GetActorRotation))
  (Utilities|IsValid (Variables|Default|GetActorNeedToBeNoticed)
    (:Is%20Valid
      (bind _rotation (Timeline|Timeline_Rotation PlayFromStart)
        (:Update
          (Transformation|SetActorRotation (Math|Rotator|Lerp(Rotator) _returnvalue (Math|Rotator|CombineRotators _returnvalue (Math|Rotator|MakeRotator 0.0 0.0 (Variables|Default|GetRotateAnglePerTime))) _rotation)))))
    (:Is%20Not%20Valid
      (Variables|Default|SetIsNoticedItemExisted false)
      (Utilities|Time|ClearandInvalidateTimerbyHandle (Variables|Default|GetCheckItemExictingTimer))
      (Actor|DestroyActor))))

(event EventBeginPlay
  (CallFunction|StartCheckIsNoticedItemExisted))

(event Collision|EventActorBeginOverlap
  (params (OtherActor :type Actor%20Object%20Reference)))

(event EventTick
  (params (DeltaSeconds :type Float%20%28single-precision%29)))

(fn ConstructionScript)