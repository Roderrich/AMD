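; Parametric storage rack furniture actor that rebuilds its shape from Size and HolderThick in the construction script.
; UpdateStorageRankSize scales six holder posts and four shelves relative to MeshReference dimensions.
; It then places the posts at the corners and mid-sides along Y, and spaces the shelves evenly at fifths of the height around a centered origin.
; All event graph events are unused, so there is no runtime logic.
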(event EventBeginPlay)

(event Collision|EventActorBeginOverlap
  (params (OtherActor :type Actor%20Object%20Reference)))

(event EventTick
  (params (DeltaSeconds :type Float%20%28single-precision%29)))

(fn ConstructionScript
  (CallFunction|UpdateStorageRankSize))

(fn UpdateStorageRankSize
  (bind _meshreference (Variables|Default|GetMeshReference))
  (bind _size (Variables|Default|GetSize))
  (bind _holderthick (Variables|Default|GetHolderThick))
  (bind _holderthick_2 (Variables|Default|GetHolderThick))
  (bind _size_2 (Variables|Default|GetSize))
  (bind _size_3 (Variables|Default|GetSize))
  (bind _size_4 (Variables|Default|GetSize))
  (bind _size_5 (Variables|Default|GetSize))
  (bind _size_6 (Variables|Default|GetSize))
  (bind _meshreference_2 (Variables|Default|GetMeshReference))
  (bind _holderthick_3 (Variables|Default|GetHolderThick))
  (bind (_x _y) (Math|Vector|BreakVector _size_6))
  (bind _z (Math|Vector|BreakVector _size_2))
  (bind _z_2 (Math|Vector|BreakVector _size_3))
  (bind _z_3 (Math|Vector|BreakVector _size_4))
  (bind (_x_2 _y_2 _z_4) (Math|Vector|BreakVector _meshreference_2))
  (bind _z_5 (Math|Vector|BreakVector _size_5))
  (bind (_x_3 _y_3 _z_6) (Math|Vector|BreakVector _meshreference))
  (bind (_x_4 _y_4) (Math|Vector|BreakVector _size))
  (bind _returnvalue (/ _holderthick_2 2.0))
  (bind _returnvalue_2 (/ _holderthick 2.0))
  (bind _returnvalue_3 (/ _y 2.0))
  (bind _returnvalue_4 (/ _x 2.0))
  (bind _returnvalue_5 (- _returnvalue_3 _returnvalue))
  (bind _returnvalue_6 (- _returnvalue_4 _returnvalue_2))
  (bind _returnvalue_7 (- 0.0 _returnvalue_6))
  (bind _returnvalue_8 (- 0.0 _returnvalue_5))
  (Utilities|FlowControl|Sequence
    (:then_0
      (Transformation|SetRelativeScale3D (Variables|Default|GetSM_Holder) (Math|Vector|MakeVector (/ _holderthick_3 _x_2) (/ _holderthick_3 _y_2) (/ (.Z (Math|Vector|BreakVector (Variables|Default|GetSize))) _z_4)))
      (Transformation|SetRelativeScale3D (Variables|Default|GetSM_Shelf1) (Math|Vector|MakeVector (/ _x_4 _x_3) (/ _y_4 _y_3) (/ (Variables|Default|GetHolderThick) _z_6))))
    (:then_1
      (Transformation|SetRelativeLocation (Variables|Default|GetSM_Holder) (Math|Vector|MakeVector _returnvalue_6 _returnvalue_5 0.0) false false)
      (Transformation|SetRelativeLocation (Variables|Default|GetSM_Holder1) (Math|Vector|MakeVector _returnvalue_7 _returnvalue_5 0.0) false false)
      (Transformation|SetRelativeLocation (Variables|Default|GetSM_Holder2) (Math|Vector|MakeVector _returnvalue_6 0.0 0.0) false false)
      (Transformation|SetRelativeLocation (Variables|Default|GetSM_Holder3) (Math|Vector|MakeVector _returnvalue_7 0.0 0.0) false false)
      (Transformation|SetRelativeLocation (Variables|Default|GetSM_Holder4) (Math|Vector|MakeVector _returnvalue_6 _returnvalue_8 0.0) false false)
      (Transformation|SetRelativeLocation (Variables|Default|GetSM_Holder5) (Math|Vector|MakeVector _returnvalue_7 _returnvalue_8 0.0) false false))
    (:then_2
      (Transformation|SetRelativeLocation (Variables|Default|GetSM_Shelf1) (Math|Vector|MakeVector 0.0 0.0 (- (* (/ _z_2 5.0) 1.0) (/ _z_2 2.0))) false false)
      (Transformation|SetRelativeLocation (Variables|Default|GetSM_Shelf2) (Math|Vector|MakeVector 0.0 0.0 (- (* (/ _z_3 5.0) 2.0) (/ _z_3 2.0))) false false)
      (Transformation|SetRelativeLocation (Variables|Default|GetSM_Shelf3) (Math|Vector|MakeVector 0.0 0.0 (- (* (/ _z_5 5.0) 3.0) (/ _z_5 2.0))) false false)
      (Transformation|SetRelativeLocation (Variables|Default|GetSM_Shelf4) (Math|Vector|MakeVector 0.0 0.0 (- (* (/ _z 5.0) 4.0) (/ _z 2.0))) false false))))