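; Interactable cabinet built from six mesh panels, with a door that opens once when the scene object is activated.
; The construction script scales and places the panels from Size, Thick and MechReference, then computes the door's closed and open transforms.
; A timeline lerps the door between those transforms, and the crosshair prompt shows until opening finishes.
; A design-time flag previews the open door in the editor, and BeginPlay resets it to closed.
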(event Custom|OpenDoor
  (if (not (Variables|Default|GetIsDoorOpened))
    (bind _dooropen (Timeline|Timeline_DoorOpen PlayFromStart)
      (:Update
        (Transformation|SetRelativeTransform (Variables|Default|GetSM_Door) (Math|Transform|Lerp(Transform) (Variables|Default|GetStartRecordRelativeTransform) (Variables|Default|GetDoorOpenTargetRelativeTransform) _dooropen) false false))
      (:Finished
        (Variables|Default|SetIsDoorOpened true)))))

(event EventBeginPlay
  (Variables|Default|SetIsCheckOpenedStateWhileDesign false)
  (Transformation|SetRelativeTransform (Variables|Default|GetSM_Door) (Variables|Default|GetStartRecordRelativeTransform) false false))

(event Collision|EventActorBeginOverlap
  (params (OtherActor :type Actor%20Object%20Reference)))

(event EventTick
  (params (DeltaSeconds :type Float%20%28single-precision%29)))

(event EventActivateSceneObject
  (CallFunction|OpenDoor))

(fn ConstructionScript
  (CallFunction|UpdateCabinetSize)
  (Transformation|SetRelativeTransform (Variables|Default|GetSM_Door) (select (Variables|Default|GetIsCheckOpenedStateWhileDesign) (Variables|Default|GetDoorOpenTargetRelativeTransform) (Variables|Default|GetStartRecordRelativeTransform)) false false))

(fn UpdateCabinetSize
  (bind _thick (Variables|Default|GetThick))
  (bind _mechreference (Variables|Default|GetMechReference))
  (bind _size (Variables|Default|GetSize))
  (bind _size_2 (Variables|Default|GetSize))
  (bind _thick_2 (Variables|Default|GetThick))
  (bind _size_3 (Variables|Default|GetSize))
  (bind _thick_3 (Variables|Default|GetThick))
  (bind _thick_4 (Variables|Default|GetThick))
  (bind _size_4 (Variables|Default|GetSize))
  (bind _size_5 (Variables|Default|GetSize))
  (bind _thick_5 (Variables|Default|GetThick))
  (bind _size_6 (Variables|Default|GetSize))
  (bind _mechreference_2 (Variables|Default|GetMechReference))
  (bind _size_7 (Variables|Default|GetSize))
  (bind _mechreference_3 (Variables|Default|GetMechReference))
  (bind _thick_6 (Variables|Default|GetThick))
  (bind _mechreference_4 (Variables|Default|GetMechReference))
  (bind _size_8 (Variables|Default|GetSize))
  (bind (_x _y _z) (Math|Vector|BreakVector _thick))
  (bind (_x_2 _y_2 _z_2) (Math|Vector|BreakVector _mechreference))
  (bind (_x_3 _y_3) (Math|Vector|BreakVector _size))
  (bind _y_4 (Math|Vector|BreakVector _size_8))
  (bind _y_5 (Math|Vector|BreakVector _thick_2))
  (bind (_x_4 _y_6) (Math|Vector|BreakVector _size_3))
  (bind _x_5 (Math|Vector|BreakVector _thick_3))
  (bind _z_3 (Math|Vector|BreakVector _size_4))
  (bind (_x_6 _y_7 _z_4) (Math|Vector|BreakVector _thick_4))
  (bind (_x_7 _y_8 _z_5) (Math|Vector|BreakVector _mechreference_3))
  (bind _x_8 (Math|Vector|BreakVector _size_5))
  (bind (_x_9 _y_9) (Math|Vector|BreakVector _thick_5))
  (bind (_x_10 _y_10 _z_6) (Math|Vector|BreakVector _size_6))
  (bind (_x_11 _y_11 _z_7) (Math|Vector|BreakVector _mechreference_2))
  (bind (_x_12 _y_12 _z_8) (Math|Vector|BreakVector _size_7))
  (bind (_x_13 _y_13) (Math|Vector|BreakVector _thick_6))
  (bind (_x_14 _y_14 _z_9) (Math|Vector|BreakVector _mechreference_4))
  (bind (_x_15 _y_15 _z_10) (Math|Vector|BreakVector _size_2))
  (bind _returnvalue (/ _y_5 2.0))
  (bind _returnvalue_2 (/ _x_4 2.0))
  (bind _returnvalue_3 (/ _z_3 2.0))
  (bind _returnvalue_4 (/ _z_4 2.0))
  (bind _returnvalue_5 (/ _y_9 2.0))
  (bind _returnvalue_6 (/ _y_7 2.0))
  (bind _returnvalue_7 (/ _x_8 2.0))
  (bind _returnvalue_8 (/ _x_9 2.0))
  (bind _returnvalue_9 (/ _y_4 2.0))
  (bind _returnvalue_10 (- _returnvalue_9 _returnvalue))
  (bind _returnvalue_11 (- _returnvalue_3 _returnvalue_4))
  (bind _returnvalue_12 (- 0.0 _returnvalue_5))
  (bind _returnvalue_13 (- 0.0 _returnvalue_6))
  (bind _returnvalue_14 (- _returnvalue_7 _returnvalue_8))
  (Utilities|FlowControl|Sequence
    (:then_0
      (Transformation|SetRelativeScale3D (Variables|Default|GetSM_Left) (Math|Vector|MakeVector (/ _x_13 _x_14) (/ (- _y_15 _y_13) _y_14) (/ _z_10 _z_9)))
      (Transformation|SetRelativeScale3D (Variables|Default|GetSM_Top) (Math|Vector|MakeVector (/ _x_3 _x_2) (/ (- _y_3 _y) _y_2) (/ _z _z_2)))
      (Transformation|SetRelativeScale3D (Variables|Default|GetSM_Back) (Math|Vector|MakeVector (/ _x_12 _x_11) (/ (.Y (Math|Vector|BreakVector (Variables|Default|GetThick))) _y_11) (/ _z_8 _z_7))))
    (:then_1
      (Transformation|SetRelativeLocation (Variables|Default|GetSM_Left) (Math|Vector|MakeVector (- 0.0 _returnvalue_14) _returnvalue_12 0.0) false false)
      (Transformation|SetRelativeLocation (Variables|Default|GetSM_Right) (Math|Vector|MakeVector _returnvalue_14 _returnvalue_12 0.0) false false)
      (Transformation|SetRelativeLocation (Variables|Default|GetSM_Top) (Math|Vector|MakeVector 0.0 _returnvalue_13 _returnvalue_11) false false)
      (Transformation|SetRelativeLocation (Variables|Default|GetSM_Down) (Math|Vector|MakeVector 0.0 _returnvalue_13 (- 0.0 _returnvalue_11)) false false)
      (Transformation|SetRelativeLocation (Variables|Default|GetSM_Back) (Math|Vector|MakeVector 0.0 (- 0.0 _returnvalue_10) 0.0) false false)
      (Transformation|SetRelativeLocation (Variables|Default|GetSM_Door) (Math|Vector|MakeVector 0.0 _returnvalue_10 0.0) false false))
    (:then_2
      (Variables|Default|SetStartRecordRelativeTransform (Transformation|GetRelativeTransform (Variables|Default|GetSM_Door)))
      (Variables|Default|SetDoorOpenTargetRelativeTransform (Math|Transform|MakeTransform (Math|Vector|MakeVector (- 0.0 (- _returnvalue_2 (/ _x_5 2.0))) (- (+ _returnvalue_2 (/ _y_6 2.0)) _x_5) 0.0) "0.000000,90.000000,0.000000" (Math|Vector|MakeVector (/ _x_10 _x_7) (/ (.Y (Math|Vector|BreakVector (Variables|Default|GetThick))) _y_8) (/ _z_6 _z_5)))))))

(fn GetAmmoInfo
  (return false "NewEnumerator0"))

(fn GetCrosshairPrompt
  (if (not (Variables|Default|GetIsDoorOpened))
    (return (Variables|Default|GetInteractionMessage) "E")))

(fn GetHealthInfo
  (return false 0.0))

(fn GetInteractionType
  (return false "NewEnumerator2"))

(fn GetIsConsumeable
  (return false))

(fn GetSceneInfo
  (return false))