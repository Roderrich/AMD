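; BP_IronNet is a procedural furniture actor that builds a crisscrossed iron lattice from stretched static meshes.
; The construction script calls UpdateIronNetSize, which tilts two base bars to opposite roll angles to form an X and scales them from the desired radius and length relative to a reference mesh size.
; It then adds more mirrored bar pairs at even spacing along Y for the configured group count, with no runtime logic.
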(event EventBeginPlay)

(event Collision|EventActorBeginOverlap
  (params (OtherActor :type Actor%20Object%20Reference)))

(event EventTick
  (params (DeltaSeconds :type Float%20%28single-precision%29)))

(fn ConstructionScript
  (CallFunction|UpdateIronNetSize))

(fn UpdateIronNetSize
  (bind _ironsizereference (Variables|Default|GetIronSizeReference))
  (bind _ironliner (Variables|Default|GetIronLineR))
  (bind _ironsizereference_2 (Variables|Default|GetIronSizeReference))
  (bind _ironliner_2 (Variables|Default|GetIronLineR))
  (bind _ironsizereference_3 (Variables|Default|GetIronSizeReference))
  (bind _ironliner_3 (Variables|Default|GetIronLineR))
  (bind _ironsizereference_4 (Variables|Default|GetIronSizeReference))
  (bind _ironliner_4 (Variables|Default|GetIronLineR))
  (bind (_x _y _z) (Math|Vector|BreakVector _ironsizereference))
  (bind (_x_2 _y_2 _z_2) (Math|Vector|BreakVector _ironsizereference_3))
  (bind (_x_3 _y_3 _z_3) (Math|Vector|BreakVector _ironsizereference_2))
  (bind (_x_4 _y_4 _z_4) (Math|Vector|BreakVector _ironsizereference_4))
  (Utilities|FlowControl|Sequence
    (:then_0
      (Transformation|SetRelativeTransform (Variables|Default|GetSM_IronLine1) (Math|Transform|MakeTransform "0, 0, 0" (Math|Rotator|MakeRotator (Variables|Default|GetAngleForALine) 0.0 0.0) (Math|Vector|MakeVector (/ _ironliner _x) (/ _ironliner _y) (/ (Variables|Default|GetIronLineLength) _z))) false false)
      (Transformation|SetRelativeTransform (Variables|Default|GetSM_IronLine2) (Math|Transform|MakeTransform "0, 0, 0" (Math|Rotator|MakeRotator (* (Variables|Default|GetAngleForALine) -1.0) 0.0 0.0) (Math|Vector|MakeVector (/ _ironliner_2 _x_3) (/ _ironliner_2 _y_3) (/ (Variables|Default|GetIronLineLength) _z_3))) false false))
    (:then_1
      (for _index (range 0 (- (Variables|Default|GetNumOfGroup) 1))
        (AddComponent|AddStaticMeshComponent false (Math|Transform|MakeTransform (Math|Vector|MakeVector 0.0 (* (+ _index 1) (Variables|Default|GetDistanceBetweenIronLine)) 0.0) (Math|Rotator|MakeRotator (Variables|Default|GetAngleForALine) 0.0 0.0) (Math|Vector|MakeVector (/ _ironliner_4 _x_4) (/ _ironliner_4 _y_4) (/ (Variables|Default|GetIronLineLength) _z_4))))
        (AddComponent|AddStaticMeshComponent false (Math|Transform|MakeTransform (Math|Vector|MakeVector 0.0 (* (+ _index 1) (Variables|Default|GetDistanceBetweenIronLine)) 0.0) (Math|Rotator|MakeRotator (* (Variables|Default|GetAngleForALine) -1.0) 0.0 0.0) (Math|Vector|MakeVector (/ _ironliner_3 _x_2) (/ _ironliner_3 _y_2) (/ (Variables|Default|GetIronLineLength) _z_2))))))))