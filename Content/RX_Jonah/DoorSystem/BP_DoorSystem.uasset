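; Automatic sliding door actor that opens when Player_RebelX enters its front or back trigger box.
; The construction script sizes and places the single or double frame, single or split retractable panels and both triggers from editable dimensions.
; Exiting a trigger closes the door after a short delay if the other is empty.
; Timelines lerp panels from their current location when IsDoorUsable is set, with a fixed Delay if an animation is still playing.
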(event OnComponentBeginOverlap(Box_Front)
  (params (OverlappedComponent :type Primitive%20Component%20Object%20Reference) (OtherActor :type Actor%20Object%20Reference) (OtherComp :type Primitive%20Component%20Object%20Reference) (OtherBodyIndex :type Integer) (bFromSweep :type Boolean) (SweepResult :type Hit%20Result%20Structure%20%28by%20ref%29))
  (Utilities|Casting|CastToPlayer_RebelX OtherActor)
  (Development|PrintString "DoorFront")
  (Variables|Default|SetInTheFrontDetectiveZone true)
  (if (not (Variables|Default|GetIsDoorOpen))
    (Variables|Default|SetIsDoorOpen true)
    (CallFunction|OpenDoor)))

(event OnComponentEndOverlap(Box_Front)
  (params (OverlappedComponent :type Primitive%20Component%20Object%20Reference) (OtherActor :type Actor%20Object%20Reference) (OtherComp :type Primitive%20Component%20Object%20Reference) (OtherBodyIndex :type Integer))
  (Utilities|Casting|CastToPlayer_RebelX OtherActor)
  (Variables|Default|SetInTheFrontDetectiveZone false)
  (Utilities|FlowControl|Delay 0.2)
  (if (not (Variables|Default|GetInTheBackDetectiveZone))
    (if (Variables|Default|GetIsDoorOpen)
      (Variables|Default|SetIsDoorOpen false)
      (CallFunction|CloseDoor))))

(event OnComponentBeginOverlap(Box_Back)
  (params (OverlappedComponent :type Primitive%20Component%20Object%20Reference) (OtherActor :type Actor%20Object%20Reference) (OtherComp :type Primitive%20Component%20Object%20Reference) (OtherBodyIndex :type Integer) (bFromSweep :type Boolean) (SweepResult :type Hit%20Result%20Structure%20%28by%20ref%29))
  (Utilities|Casting|CastToPlayer_RebelX OtherActor)
  (Variables|Default|SetInTheBackDetectiveZone true)
  (if (not (Variables|Default|GetIsDoorOpen))
    (Variables|Default|SetIsDoorOpen true)
    (CallFunction|OpenDoor)))

(event OnComponentEndOverlap(Box_Back)
  (params (OverlappedComponent :type Primitive%20Component%20Object%20Reference) (OtherActor :type Actor%20Object%20Reference) (OtherComp :type Primitive%20Component%20Object%20Reference) (OtherBodyIndex :type Integer))
  (Utilities|Casting|CastToPlayer_RebelX OtherActor)
  (Variables|Default|SetInTheBackDetectiveZone false)
  (Utilities|FlowControl|Delay 0.2)
  (if (not (Variables|Default|GetInTheFrontDetectiveZone))
    (if (Variables|Default|GetIsDoorOpen)
      (Variables|Default|SetIsDoorOpen false)
      (CallFunction|CloseDoor))))

(event Custom|OpenDoor
  (bind _sm_door_singlesidedretractable (Variables|Default|GetSM_Door_SingleSidedRetractable))
  (bind _sm_door_doublesidedretractable1 (Variables|Default|GetSM_Door_DoubleSidedRetractable1))
  (bind _sm_door_doublesidedretractable2 (Variables|Default|GetSM_Door_DoubleSidedRetractable2))
  (bind _relativelocation (Variables|/Script/Engine.SceneComponent|GetRelativeLocation _sm_door_singlesidedretractable))
  (bind _relativelocation_2 (Variables|/Script/Engine.SceneComponent|GetRelativeLocation _sm_door_doublesidedretractable1))
  (bind _relativelocation_3 (Variables|/Script/Engine.SceneComponent|GetRelativeLocation _sm_door_doublesidedretractable2))
  (bind (_x _y _z) (Math|Vector|BreakVector _relativelocation))
  (bind (_x_2 _y_2 _z_2) (Math|Vector|BreakVector _relativelocation_2))
  (bind (_x_3 _y_3 _z_3) (Math|Vector|BreakVector _relativelocation_3))
  (if (not (Variables|Default|GetIsPreviousAnimationIsPlaying))
    _
    (else
      (Utilities|FlowControl|Delay 1.05)))
  (Variables|Default|SetIsPreviousAnimationIsPlaying true)
  (if (Variables|Default|GetIsDoorUsable)
    (switch Utilities|FlowControl|Switch|SwitchonE_DoorOpenType (Variables|Default|GetDoorType)
      (:NewEnumerator1
        (bind _retractabledoor (Timeline|Timeline_SingleSidedRetractableDoorOpen PlayFromStart)
          (:Update
            (Transformation|SetRelativeLocation (Variables|Default|GetSM_Door_SingleSidedRetractable) (Math|Vector|Lerp(Vector) (Variables|/Script/Engine.SceneComponent|GetRelativeLocation (Variables|Default|GetSM_Door_SingleSidedRetractable)) (Math|Vector|MakeVector (- 0.0 (.X (Math|Vector|BreakVector (Variables|Default|GetDoorSize)))) _y _z) _retractabledoor) false false))
          (:Finished
            (Variables|Default|SetIsPreviousAnimationIsPlaying false))))
      (:NewEnumerator2
        (bind _retractabledoor_2 (Timeline|Timeline_DoubleSidedRetractableDoorOpen PlayFromStart)
          (:Update
            (Transformation|SetRelativeLocation (Variables|Default|GetSM_Door_DoubleSidedRetractable1) (Math|Vector|Lerp(Vector) (Variables|/Script/Engine.SceneComponent|GetRelativeLocation (Variables|Default|GetSM_Door_DoubleSidedRetractable1)) (Math|Vector|MakeVector (- 0.0 (.X (Math|Vector|BreakVector (Variables|Default|GetDoorSize)))) _y_2 _z_2) _retractabledoor_2) false false)
            (Transformation|SetRelativeLocation (Variables|Default|GetSM_Door_DoubleSidedRetractable2) (Math|Vector|Lerp(Vector) (Variables|/Script/Engine.SceneComponent|GetRelativeLocation (Variables|Default|GetSM_Door_DoubleSidedRetractable2)) (Math|Vector|MakeVector (.X (Math|Vector|BreakVector (Variables|Default|GetDoorSize))) _y_3 _z_3) _retractabledoor_2) false false))
          (:Finished
            (Variables|Default|SetIsPreviousAnimationIsPlaying false)))))))

(event Custom|CloseDoor
  (if (not (Variables|Default|GetIsPreviousAnimationIsPlaying))
    _
    (else
      (Utilities|FlowControl|Delay 1.05)))
  (Variables|Default|SetIsPreviousAnimationIsPlaying true)
  (if (Variables|Default|GetIsDoorUsable)
    (switch Utilities|FlowControl|Switch|SwitchonE_DoorOpenType (Variables|Default|GetDoorType)
      (:NewEnumerator1
        (bind _retractabledoor (Timeline|Timeline_SingleSidedRetractableDoorClose PlayFromStart)
          (:Update
            (Transformation|SetRelativeLocation (Variables|Default|GetSM_Door_SingleSidedRetractable) (Math|Vector|Lerp(Vector) (Variables|/Script/Engine.SceneComponent|GetRelativeLocation (Variables|Default|GetSM_Door_SingleSidedRetractable)) (Variables|Default|GetDoorClosedRelativeLocation1) _retractabledoor) false false))
          (:Finished
            (Variables|Default|SetIsPreviousAnimationIsPlaying false))))
      (:NewEnumerator2
        (bind _retractabledoor_2 (Timeline|Timeline_DoubleSidedRetractableDoorClose PlayFromStart)
          (:Update
            (Transformation|SetRelativeLocation (Variables|Default|GetSM_Door_DoubleSidedRetractable1) (Math|Vector|Lerp(Vector) (Variables|/Script/Engine.SceneComponent|GetRelativeLocation (Variables|Default|GetSM_Door_DoubleSidedRetractable1)) (Variables|Default|GetDoorClosedRelativeLocation1) _retractabledoor_2) false false)
            (Transformation|SetRelativeLocation (Variables|Default|GetSM_Door_DoubleSidedRetractable2) (Math|Vector|Lerp(Vector) (Variables|/Script/Engine.SceneComponent|GetRelativeLocation (Variables|Default|GetSM_Door_DoubleSidedRetractable2)) (Variables|Default|GetDoorClosedRelativeLocation2) _retractabledoor_2) false false))
          (:Finished
            (Variables|Default|SetIsPreviousAnimationIsPlaying false)))))))

(event EventBeginPlay
  (switch Utilities|FlowControl|Switch|SwitchonE_DoorOpenType (Variables|Default|GetDoorType)
    (:NewEnumerator1
      (Variables|Default|SetDoorClosedRelativeLocation1 (Variables|/Script/Engine.SceneComponent|GetRelativeLocation (Variables|Default|GetSM_Door_SingleSidedRetractable)))
      (Collision|SetCollisionResponsetoChannel (Variables|Default|GetSM_Door_SingleSidedRetractable) "ECC_Pawn" "ECR_Block"))
    (:NewEnumerator2
      (Variables|Default|SetDoorClosedRelativeLocation1 (Variables|/Script/Engine.SceneComponent|GetRelativeLocation (Variables|Default|GetSM_Door_DoubleSidedRetractable1)))
      (Variables|Default|SetDoorClosedRelativeLocation2 (Variables|/Script/Engine.SceneComponent|GetRelativeLocation (Variables|Default|GetSM_Door_DoubleSidedRetractable2)))
      (Collision|SetCollisionResponsetoChannel (Variables|Default|GetSM_Door_DoubleSidedRetractable1) "ECC_Pawn" "ECR_Block"))))

(event Collision|EventActorBeginOverlap
  (params (OtherActor :type Actor%20Object%20Reference)))

(event EventTick
  (params (DeltaSeconds :type Float%20%28single-precision%29)))

(fn ConstructionScript
  (CallFunction|UpdateDoorMesh))

(fn UpdateDoorMesh
  (bind _doorframesize (Variables|Default|GetDoorFrameSize))
  (bind _sm__doorjamb1_2 (Variables|Default|GetSM%20_DoorJamb1-2))
  (bind _doorframedepthifdouble (Variables|Default|GetDoorFrameDepthIfDouble))
  (bind _doorframesize_2 (Variables|Default|GetDoorFrameSize))
  (bind _doorframedepthifdouble_2 (Variables|Default|GetDoorFrameDepthIfDouble))
  (bind _sm_door_singlesidedretractable (Variables|Default|GetSM_Door_SingleSidedRetractable))
  (bind _sm__doorjamb1 (Variables|Default|GetSM%20_DoorJamb1))
  (bind _sizereference (Variables|Default|GetSizeReference))
  (bind _sm_door_singlesidedretractable_2 (Variables|Default|GetSM_Door_SingleSidedRetractable))
  (bind _doorsize (Variables|Default|GetDoorSize))
  (bind _sizereference_2 (Variables|Default|GetSizeReference))
  (bind _doorframesize_3 (Variables|Default|GetDoorFrameSize))
  (bind _doorframesize_4 (Variables|Default|GetDoorFrameSize))
  (bind _sizereference_3 (Variables|Default|GetSizeReference))
  (bind _doorsize_2 (Variables|Default|GetDoorSize))
  (bind _sm_door_doublesidedretractable1 (Variables|Default|GetSM_Door_DoubleSidedRetractable1))
  (bind _doorsize_3 (Variables|Default|GetDoorSize))
  (bind _sizereference_4 (Variables|Default|GetSizeReference))
  (bind _doorsize_4 (Variables|Default|GetDoorSize))
  (bind _sm__doorjamb1_2_2 (Variables|Default|GetSM%20_DoorJamb1-2))
  (bind _sizereference_5 (Variables|Default|GetSizeReference))
  (bind _sizereference_6 (Variables|Default|GetSizeReference))
  (bind (_x _y _z) (Math|Vector|BreakVector _sizereference_2))
  (bind _y_2 (Math|Vector|BreakVector _doorframesize))
  (bind _y_3 (Math|Vector|BreakVector _doorframesize_2))
  (bind (_x_2 _y_4 _z_2) (Math|Vector|BreakVector _sizereference))
  (bind (_x_3 _y_5 _z_3) (Math|Vector|BreakVector _doorsize))
  (bind _z_4 (Math|Vector|BreakVector _doorframesize_3))
  (bind (_x_4 _y_6 _z_5) (Math|Vector|BreakVector _doorframesize_4))
  (bind (_x_5 _y_7) (Math|Vector|BreakVector _sizereference_4))
  (bind (_x_6 _y_8 _z_6) (Math|Vector|BreakVector _doorsize_2))
  (bind (_x_7 _y_9 _z_7) (Math|Vector|BreakVector _sizereference_3))
  (bind (_x_8 _y_10 _z_8) (Math|Vector|BreakVector _doorsize_3))
  (bind (_x_9 _y_11 _z_9) (Math|Vector|BreakVector _doorsize_4))
  (bind (_x_10 _y_12) (Math|Vector|BreakVector _sizereference_5))
  (bind (_x_11 _y_13 _z_10) (Math|Vector|BreakVector _sizereference_6))
  (bind _returnvalue (/ _doorframedepthifdouble 2.0))
  (bind _returnvalue_2 (/ _doorframedepthifdouble_2 2.0))
  (bind _returnvalue_3 (/ _z_4 2.0))
  (bind _returnvalue_4 (/ _y_2 2.0))
  (bind _returnvalue_5 (/ _y_3 2.0))
  (bind _returnvalue_6 (- _returnvalue_4 _returnvalue))
  (bind _returnvalue_7 (- _returnvalue_5 _returnvalue_2))
  (bind _returnvalue_8 (- 0.0 _returnvalue_7))
  (Utilities|FlowControl|Sequence ; 0 DoorFrame\n1 Door\n2 DoorCollision
    (:then_0
      (Collision|SetCollisionEnabled _sm__doorjamb1_2 "NoCollision")
      (Rendering|SetVisibility _sm__doorjamb1_2 false false)
      (Development|SetHiddeninGame (Variables|Default|GetSM%20_DoorHeadJamb2) true false)
      (Collision|SetCollisionResponsetoChannel _sm__doorjamb1_2 "ECC_Pawn" "ECR_Ignore")
      (if (Variables|Default|GetIsUseDoubleFrame)
        (Collision|SetCollisionEnabled _sm__doorjamb1_2_2 "QueryAndPhysics")
        (Rendering|SetVisibility _sm__doorjamb1_2_2 true false)
        (Development|SetHiddeninGame (Variables|Default|GetSM%20_DoorHeadJamb2) false false)
        (Collision|SetCollisionResponsetoChannel _sm__doorjamb1_2_2 "ECC_Pawn" "ECR_Block")
        (Utilities|FlowControl|Sequence ; 0 Relative Scale\n1 Relative Location
          (:then_0
            (Transformation|SetRelativeScale3D (Variables|Default|GetSM%20_DoorJamb1) (Math|Vector|MakeVector (/ (Variables|Default|GetDoorFrameThickness) _x_5) (/ (Variables|Default|GetDoorFrameDepthIfDouble) _y_7) (/ (.Z (Math|Vector|BreakVector (Variables|Default|GetDoorFrameSize))) (.Z (Math|Vector|BreakVector (Variables|Default|GetSizeReference))))))
            (Transformation|SetRelativeScale3D (Variables|Default|GetSM%20_DoorHeadJamb) (Math|Vector|MakeVector (/ (.X (Math|Vector|BreakVector (Variables|Default|GetDoorFrameSize))) (.X (Math|Vector|BreakVector (Variables|Default|GetSizeReference)))) (/ (Variables|Default|GetDoorFrameDepthIfDouble) _y) (/ (Variables|Default|GetDoorFrameThickness) _z))))
          (:then_1
            (Transformation|SetRelativeLocation (Variables|Default|GetSM%20_DoorJamb1) (Math|Vector|MakeVector (- 0.0 (- (/ (.X (Math|Vector|BreakVector (Variables|Default|GetDoorFrameSize))) 2.0) (/ (Variables|Default|GetDoorFrameThickness) 2.0))) _returnvalue_8 (/ (.Z (Math|Vector|BreakVector (Variables|Default|GetDoorFrameSize))) 2.0)) false false)
            (Transformation|SetRelativeLocation (Variables|Default|GetSM%20_DoorJamb2) (Math|Vector|MakeVector (- (/ (.X (Math|Vector|BreakVector (Variables|Default|GetDoorFrameSize))) 2.0) (/ (Variables|Default|GetDoorFrameThickness) 2.0)) _returnvalue_8 (/ (.Z (Math|Vector|BreakVector (Variables|Default|GetDoorFrameSize))) 2.0)) false false)
            (Transformation|SetRelativeLocation (Variables|Default|GetSM%20_DoorHeadJamb) (Math|Vector|MakeVector 0.0 _returnvalue_8 (- (.Z (Math|Vector|BreakVector (Variables|Default|GetDoorFrameSize))) (/ (Variables|Default|GetDoorFrameThickness) 2.0))) false false)
            (Transformation|SetRelativeLocation (Variables|Default|GetSM%20_DoorJamb1-2) (Math|Vector|MakeVector (- 0.0 (- (/ (.X (Math|Vector|BreakVector (Variables|Default|GetDoorFrameSize))) 2.0) (/ (Variables|Default|GetDoorFrameThickness) 2.0))) _returnvalue_6 (/ (.Z (Math|Vector|BreakVector (Variables|Default|GetDoorFrameSize))) 2.0)) false false)
            (Transformation|SetRelativeLocation (Variables|Default|GetSM%20_DoorJamb2-2) (Math|Vector|MakeVector (- (/ (.X (Math|Vector|BreakVector (Variables|Default|GetDoorFrameSize))) 2.0) (/ (Variables|Default|GetDoorFrameThickness) 2.0)) _returnvalue_6 (/ (.Z (Math|Vector|BreakVector (Variables|Default|GetDoorFrameSize))) 2.0)) false false)
            (Transformation|SetRelativeLocation (Variables|Default|GetSM%20_DoorHeadJamb2) (Math|Vector|MakeVector 0.0 _returnvalue_6 (- (.Z (Math|Vector|BreakVector (Variables|Default|GetDoorFrameSize))) (/ (Variables|Default|GetDoorFrameThickness) 2.0))) false false)))
        (else
          (Collision|SetCollisionEnabled (Variables|Default|GetSM%20_DoorHeadJamb) "QueryAndPhysics")
          (Rendering|SetVisibility _sm__doorjamb1 true false)
          (Development|SetHiddeninGame _sm__doorjamb1 false false)
          (Collision|SetCollisionResponsetoChannel _sm__doorjamb1 "ECC_Pawn" "ECR_Block")
          (Utilities|FlowControl|Sequence ; 0 Relative Scale\n1 Relative Location
            (:then_0
              (Transformation|SetRelativeScale3D (Variables|Default|GetSM%20_DoorJamb1) (Math|Vector|MakeVector (/ (Variables|Default|GetDoorFrameThickness) _x_10) (/ (.Y (Math|Vector|BreakVector (Variables|Default|GetDoorFrameSize))) _y_12) (/ (.Z (Math|Vector|BreakVector (Variables|Default|GetDoorFrameSize))) (.Z (Math|Vector|BreakVector (Variables|Default|GetSizeReference))))))
              (Transformation|SetRelativeScale3D (Variables|Default|GetSM%20_DoorHeadJamb) (Math|Vector|MakeVector (/ (.X (Math|Vector|BreakVector (Variables|Default|GetDoorFrameSize))) (.X (Math|Vector|BreakVector (Variables|Default|GetSizeReference)))) (/ (.Y (Math|Vector|BreakVector (Variables|Default|GetDoorFrameSize))) _y_13) (/ (Variables|Default|GetDoorFrameThickness) _z_10))))
            (:then_1
              (Transformation|SetRelativeLocation (Variables|Default|GetSM%20_DoorJamb1) (Math|Vector|MakeVector (- 0.0 (- (/ (.X (Math|Vector|BreakVector (Variables|Default|GetDoorFrameSize))) 2.0) (/ (Variables|Default|GetDoorFrameThickness) 2.0))) 0.0 (/ (.Z (Math|Vector|BreakVector (Variables|Default|GetDoorFrameSize))) 2.0)) false false)
              (Transformation|SetRelativeLocation (Variables|Default|GetSM%20_DoorJamb2) (Math|Vector|MakeVector (- (/ (.X (Math|Vector|BreakVector (Variables|Default|GetDoorFrameSize))) 2.0) (/ (Variables|Default|GetDoorFrameThickness) 2.0)) 0.0 (/ (.Z (Math|Vector|BreakVector (Variables|Default|GetDoorFrameSize))) 2.0)) false false)
              (Transformation|SetRelativeLocation (Variables|Default|GetSM%20_DoorHeadJamb) (Math|Vector|MakeVector 0.0 0.0 (- (.Z (Math|Vector|BreakVector (Variables|Default|GetDoorFrameSize))) (/ (Variables|Default|GetDoorFrameThickness) 2.0))) false false))))))
    (:then_1
      (Rendering|SetVisibility (Variables|Default|GetSM_Door_SingleSidedRetractable) false false)
      (Development|SetHiddeninGame _sm_door_singlesidedretractable true false)
      (Collision|SetCollisionEnabled _sm_door_singlesidedretractable "NoCollision")
      (Collision|SetCollisionResponsetoChannel _sm_door_singlesidedretractable "ECC_Pawn" "ECR_Ignore")
      (switch Utilities|FlowControl|Switch|SwitchonE_DoorOpenType (Variables|Default|GetDoorType)
        (:NewEnumerator1
          (Rendering|SetVisibility _sm_door_singlesidedretractable_2 true false)
          (Development|SetHiddeninGame _sm_door_singlesidedretractable_2 false false)
          (Collision|SetCollisionEnabled _sm_door_singlesidedretractable_2 "QueryAndPhysics")
          (Collision|SetCollisionResponsetoChannel _sm_door_singlesidedretractable_2 "ECC_Pawn" "ECR_Block")
          (Utilities|FlowControl|Sequence ; 0 Relative Scale\n1 Relative Location
            (:then_0
              (Transformation|SetRelativeScale3D (Variables|Default|GetSM_Door_SingleSidedRetractable) (Math|Vector|MakeVector (/ _x_6 _x_7) (/ _y_8 _y_9) (/ _z_6 _z_7))))
            (:then_1
              (Transformation|SetRelativeLocation (Variables|Default|GetSM_Door_SingleSidedRetractable) (Math|Vector|MakeVector 0.0 0.0 (/ (.Z (Math|Vector|BreakVector (Variables|Default|GetDoorSize))) 2.0)) false false))))
        (:NewEnumerator2
          (Rendering|SetVisibility _sm_door_doublesidedretractable1 true false)
          (Development|SetHiddeninGame _sm_door_doublesidedretractable1 false false)
          (Collision|SetCollisionEnabled _sm_door_doublesidedretractable1 "QueryAndPhysics")
          (Collision|SetCollisionResponsetoChannel _sm_door_doublesidedretractable1 "ECC_Pawn" "ECR_Block")
          (Utilities|FlowControl|Sequence ; 0 Relative Scale\n1 Relative Location
            (:then_0
              (Transformation|SetRelativeScale3D (Variables|Default|GetSM_Door_DoubleSidedRetractable1) (Math|Vector|MakeVector (Utilities|Operators|Divide _x_8 _x_2 2.0) (/ _y_10 _y_4) (/ _z_8 _z_2))))
            (:then_1
              (Transformation|SetRelativeLocation (Variables|Default|GetSM_Door_DoubleSidedRetractable1) (Math|Vector|MakeVector (- 0.0 (/ _x_9 4.0)) 0.0 (/ _z_9 2.0)) false false)
              (Transformation|SetRelativeLocation (Variables|Default|GetSM_Door_DoubleSidedRetractable2) (Math|Vector|MakeVector (/ _x_3 4.0) 0.0 (/ _z_3 2.0)) false false))))))
    (:then_2
      (Components|Box|SetBoxExtent (Variables|Default|GetBox_Front) (Math|Vector|MakeVectorNetQuantize (/ _x_4 2.0) (/ (Variables|Default|GetDoorDetectDistance) 2.0) (/ _z_5 2.0)) true)
      (Transformation|SetRelativeLocation (Variables|Default|GetBox_Front) (Math|Vector|MakeVectorNetQuantize 0.0 (/ (Variables|Default|GetDoorDetectDistance) 2.0) _returnvalue_3) false false)
      (Transformation|SetRelativeLocation (Variables|Default|GetBox_Back) (Math|Vector|MakeVector 0.0 (- 0.0 (/ (Variables|Default|GetDoorDetectDistance) 2.0)) _returnvalue_3) false false))))