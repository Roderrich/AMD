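; BP_LaserRoomSystem manages a laser room hazard: a heavy-damage wall that sweeps back and forth between two transforms.
; SpawnLaserWall creates or reuses a BP_Damage_Volume at the start transform and configures its rapid damage ticks.
; MoveLaserWall alternates two timelines that lerp its location, re-calling itself at each end until StopAndRemoveLaserWall halts and destroys it.
; BeginPlay applies MovingSpeed only to the return timeline and does not start the wall.
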(event Custom|SpawnLaserWall
  (Utilities|IsValid (Variables|Default|GetLaserWall)
    (:Is%20Valid
      _)
    (:Is%20Not%20Valid
      (bind _returnvalue (Game|SpawnActorfromClass "/Game/RebelX_Core/_Useable/BP_Damage_Volume.BP_Damage_Volume_C" (Math|Transform|MakeTransform "0, 0, 0" "0, 0, 0" "1.000000,1.000000,1.000000") "Undefined" "MultiplyWithRoot" 0 0))
      (Variables|Default|SetLaserWall _returnvalue)))
  (Transformation|SetActorTransform (Variables|Default|GetLaserWall) (Variables|Default|GetLaserStartTransform))
  (Variables|/Game/RebelX_Core/_Useable/BP_Damage_Volume.BP_Damage_Volume_C|SetDamage%20Tick%20Duration (Variables|Default|GetLaserWall) 0.01)
  (Variables|/Game/RebelX_Core/_Useable/BP_Damage_Volume.BP_Damage_Volume_C|SetDamage%20Per%20Tick (Variables|Default|GetLaserWall) 5e+02)
  (Variables|Default|SetIsReachToStartPoint true))

(event Custom|MoveLaserWall
  (Utilities|IsValid (Variables|Default|GetLaserWall)
    (:Is%20Valid
      _)
    (:Is%20Not%20Valid
      (CallFunction|SpawnLaserWall)))
  (if (Variables|Default|GetIsReachToStartPoint)
    (bind _laserwallmovespeed (Timeline|Timeline_LaserMovingFromStartToEnd PlayFromStart)
      (:Update
        (Transformation|SetActorLocation (Variables|Default|GetLaserWall) (Math|Vector|Lerp(Vector) (.Location (Math|Transform|BreakTransform (Variables|Default|GetLaserStartTransform))) (.Location (Math|Transform|BreakTransform (Variables|Default|GetLaserEndTransform))) _laserwallmovespeed) false false))
      (:Finished
        (Utilities|FlowControl|Sequence
          (:then_0
            (Timeline|Timeline_LaserMovingFromStartToEnd Stop))
          (:then_1
            (Variables|Default|SetIsReachToStartPoint false)
            (CallFunction|MoveLaserWall)))))
    (else
      (bind _laserwallmovespeed_2 (Timeline|Timeline_LaserMovingFromEndToStart PlayFromStart)
        (:Update
          (Transformation|SetActorLocation (Variables|Default|GetLaserWall) (Math|Vector|Lerp(Vector) (.Location (Math|Transform|BreakTransform (Variables|Default|GetLaserEndTransform))) (.Location (Math|Transform|BreakTransform (Variables|Default|GetLaserStartTransform))) _laserwallmovespeed_2) false false))
        (:Finished
          (Utilities|FlowControl|Sequence
            (:then_0
              (Timeline|Timeline_LaserMovingFromEndToStart Stop))
            (:then_1
              (Variables|Default|SetIsReachToStartPoint true)
              (CallFunction|MoveLaserWall))))))))

(event Custom|StopAndRemoveLaserWall
  (Audio|Components|Audio|Stop (Variables|Default|GetTimeline_LaserMovingFromEndToStart))
  (Actor|DestroyActor (Variables|Default|GetLaserWall)))

(event EventBeginPlay
  (Components|Timeline|SetPlayRate (Variables|Default|GetTimeline_LaserMovingFromEndToStart) (Variables|Default|GetMovingSpeed)))

(fn ConstructionScript)