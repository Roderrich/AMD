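; Boss laser weapon that fires a Niagara beam along its pointer mesh's forward vector and damages the Player_RebelX character.
; IsActiveLaser shows or hides the beam and starts or stops a fast looping timer that runs the line trace.
; Each trace sets the beam length and applies heavy damage to a player hit, throttled by a DoOnce and delay cooldown.
; TargetPlayer only gates tracing, shutting the laser off when invalid.
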(event Custom|IsActiveLaser
  (params (IsActiveLaser :type Boolean))
  (bind _niagara_laser (Variables|Default|GetNiagara_Laser))
  (bind _output_get (Variables|Default|SetIsLineTraceActivated IsActiveLaser))
  (if _output_get
    (Rendering|SetVisibility _niagara_laser true false)
    (CallFunction|StartLaserLineTrace)
    (else
      (Rendering|SetVisibility _niagara_laser false false)
      (CallFunction|StopLaserLineTrace))))

(event Custom|LaserLineTrace
  (bind _sm_laserpointer (Variables|Default|GetSM_LaserPointer))
  (bind _laserlinetracemaxdistance (Variables|Default|GetLaserLineTraceMaxDistance))
  (bind _returnvalue (Transformation|GetWorldLocation _sm_laserpointer))
  (Utilities|IsValid (Variables|Default|GetTargetPlayer)
    (:Is%20Valid
      (bind (_outhit _returnvalue_2) (Collision|LineTraceByChannel _returnvalue (+ _returnvalue (* (Math|Vector|GetForwardVector _sm_laserpointer) _laserlinetracemaxdistance)) "TraceTypeQuery4" false 0 "None"))
      (if _returnvalue_2
        (Effects|Components|ParticleSystem|SetVectorParameter (Variables|Default|GetNiagara_Laser) "Beam End" (Math|Vector|MakeVector (.Distance (Collision|BreakHitResult _outhit)) 0.0 0.0))
        (bind _asplayer_rebel_x (Utilities|Casting|CastToPlayer_RebelX (.HitActor (Collision|BreakHitResult _outhit))))
        (Utilities|FlowControl|DoOnce false :!label _label
          (:Completed
            (Game|Damage|ApplyDamage _asplayer_rebel_x 1.7e+02 0 0)
            (Utilities|FlowControl|Delay 2.0)
            (goto _label Reset)))
        (else
          (Effects|Components|ParticleSystem|SetVectorParameter (Variables|Default|GetNiagara_Laser) "Beam End" (Math|Vector|MakeVector _laserlinetracemaxdistance 0.0 0.0)))))
    (:Is%20Not%20Valid
      (CallFunction|IsActiveLaser false))))

(event Custom|StartLaserLineTrace
  (bind _returnvalue (Utilities|Time|SetTimerbyEvent (delegate Custom|LaserLineTrace) 0.01 true))
  (Variables|Default|SetLaserLineTraceTimer _returnvalue))

(event Custom|StopLaserLineTrace
  (Utilities|Time|ClearandInvalidateTimerbyHandle (Variables|Default|GetLaserLineTraceTimer)))

(event EventBeginPlay
  (Utilities|FlowControl|Sequence
    (:then_0
      (Rendering|SetVisibility (Variables|Default|GetNiagara_Laser) false false))))

(fn ConstructionScript)

(fn SetTargetPlayer
  (params (Target :type Player%20Rebel%20X%20Object%20Reference))
  (Variables|Default|SetTargetPlayer Target))