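; Boss projectile that flies in a straight line and deals fixed damage to the Player_RebelX it hits.
; On BeginPlay it configures overlap collision, then a timeline paced by BulletSpeed lerps it from StartTransform along the direction of TargetTransform for a fixed distance, extending beyond or short of the target.
; It destroys itself on any collision overlap or when the timeline finishes.
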(event OnComponentBeginOverlap(BulletCollision)
  (params (OverlappedComponent :type Primitive%20Component%20Object%20Reference) (OtherActor :type Actor%20Object%20Reference) (OtherComp :type Primitive%20Component%20Object%20Reference) (OtherBodyIndex :type Integer) (bFromSweep :type Boolean) (SweepResult :type Hit%20Result%20Structure%20%28by%20ref%29))
  (bind _asplayer_rebel_x (Utilities|Casting|CastToPlayer_RebelX OtherActor)
    (:then
      (Game|Damage|ApplyDamage _asplayer_rebel_x 3e+01 0 self)
      (Actor|DestroyActor))
    (:CastFailed
      (Actor|DestroyActor))))

(event EventBeginPlay
  (bind _bulletcollision (Variables|Default|GetBulletCollision))
  (bind _targettransform (Variables|Default|GetTargetTransform))
  (bind (_location _rotation _scale) (Math|Transform|BreakTransform _targettransform))
  (Collision|SetCollisionEnabled _bulletcollision "QueryAndPhysics")
  (Collision|SetCollisionResponsetoAllChannels _bulletcollision "ECR_Overlap")
  (Collision|SetCollisionResponsetoChannel _bulletcollision "ECC_GameTraceChannel7" "ECR_Ignore")
  (Collision|SetCollisionResponsetoChannel _bulletcollision "ECC_GameTraceChannel8" "ECR_Ignore")
  (Collision|SetCollisionResponsetoChannel _bulletcollision "ECC_Pawn" "ECR_Overlap")
  (Variables|Default|SetDeltaTransform (Math|Transform|MakeTransform (* (Math|Vector|Normalize (- (.Location (Math|Transform|BreakTransform (Variables|Default|GetTargetTransform))) (.Location (Math|Transform|BreakTransform (Variables|Default|GetStartTransform))))) 3e+03) _rotation _scale))
  (Components|Timeline|SetPlayRate (Variables|Default|GetTimeline_MoveToTargetTransform) (Variables|Default|GetBulletSpeed))
  (bind _newtrack_0 (Timeline|Timeline_MoveToTargetTransform PlayFromStart)
    (:Update
      (Transformation|SetActorTransform (Math|Transform|Lerp(Transform) (Variables|Default|GetStartTransform) (Math|Transform|MakeTransform (+ (.Location (Math|Transform|BreakTransform (Variables|Default|GetStartTransform))) (.Location (Math|Transform|BreakTransform (Variables|Default|GetDeltaTransform)))) (.Rotation (Math|Transform|BreakTransform (Variables|Default|GetDeltaTransform))) (.Scale (Math|Transform|BreakTransform (Variables|Default|GetDeltaTransform)))) _newtrack_0)))
    (:Finished
      (Actor|DestroyActor))))

(event Collision|EventActorBeginOverlap
  (params (OtherActor :type Actor%20Object%20Reference)))

(event EventTick
  (params (DeltaSeconds :type Float%20%28single-precision%29)))

(fn ConstructionScript)