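; Elevator actor whose cabin is sized in the editor from five pieces: two side walls, back wall, floor and ceiling.
; The construction script scales each piece from ElevatorSize and WallThickness relative to SizeReference, then offsets it around the center.
; A separate function, not called here, copies each linked floor caller's target transform into a floor-keyed map.
; Event graph stubs are empty, so no movement logic exists here.
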(event EventBeginPlay)

(event Collision|EventActorBeginOverlap
  (params (OtherActor :type Actor%20Object%20Reference)))

(event EventTick
  (params (DeltaSeconds :type Float%20%28single-precision%29)))

(fn ConstructionScript
  (CallFunction|UpdateElevatorAppearance))

(fn UpdateElevatorAppearance
  (bind _sizereference (Variables|Default|GetSizeReference))
  (bind _elevator_rightwall (Variables|Default|GetElevator_RightWall))
  (bind _elevatorsize (Variables|Default|GetElevatorSize))
  (bind _sizereference_2 (Variables|Default|GetSizeReference))
  (bind _elevator_ceiling (Variables|Default|GetElevator_Ceiling))
  (bind _elevator_floor (Variables|Default|GetElevator_Floor))
  (bind _elevatorsize_2 (Variables|Default|GetElevatorSize))
  (bind _sizereference_3 (Variables|Default|GetSizeReference))
  (bind _elevator_backwall (Variables|Default|GetElevator_BackWall))
  (bind _elevatorsize_3 (Variables|Default|GetElevatorSize))
  (bind _sizereference_4 (Variables|Default|GetSizeReference))
  (bind _sizereference_5 (Variables|Default|GetSizeReference))
  (bind _elevatorsize_4 (Variables|Default|GetElevatorSize))
  (bind _elevatorsize_5 (Variables|Default|GetElevatorSize))
  (bind _elevator_leftwall (Variables|Default|GetElevator_LeftWall))
  (bind (_x _y _z) (Math|Vector|BreakVector _elevatorsize_4))
  (bind (_x_2 _y_2 _z_2) (Math|Vector|BreakVector _sizereference))
  (bind (_x_3 _y_3 _z_3) (Math|Vector|BreakVector _elevatorsize))
  (bind (_x_4 _y_4 _z_4) (Math|Vector|BreakVector _sizereference_2))
  (bind (_x_5 _y_5 _z_5) (Math|Vector|BreakVector _elevatorsize_2))
  (bind (_x_6 _y_6) (Math|Vector|BreakVector _sizereference_3))
  (bind (_x_7 _y_7 _z_6) (Math|Vector|BreakVector _elevatorsize_3))
  (bind (_x_8 _y_8) (Math|Vector|BreakVector _sizereference_4))
  (bind (_x_9 _y_9 _z_7) (Math|Vector|BreakVector _sizereference_5))
  (bind (_x_10 _y_10 _z_8) (Math|Vector|BreakVector _elevatorsize_5))
  (Utilities|FlowControl|Sequence ; 0 Left wall\n1 Right Wall\n2 Bottom Floor\n3 Top Ceiling\n4 Back Wall\n5
    (:then_0
      (Transformation|SetRelativeScale3D _elevator_leftwall (Math|Vector|MakeVector (/ (Variables|Default|GetWallThickness) (.X (Math|Vector|BreakVector (Variables|Default|GetSizeReference)))) (/ _y_10 _y_2) (/ _z_8 _z_2)))
      (Transformation|SetRelativeLocation _elevator_leftwall (Math|Vector|MakeVector (* (/ _x_10 2.0) -1.0) 0.0 0.0) false false))
    (:then_1
      (Transformation|SetRelativeScale3D _elevator_rightwall (Math|Vector|MakeVector (/ (Variables|Default|GetWallThickness) (.X (Math|Vector|BreakVector (Variables|Default|GetSizeReference)))) (/ _y_3 _y_4) (/ _z_3 _z_4)))
      (Transformation|SetRelativeLocation _elevator_rightwall (Math|Vector|MakeVector (/ _x_3 2.0) 0.0 0.0) false false))
    (:then_2
      (Transformation|SetRelativeScale3D _elevator_floor (Math|Vector|MakeVector (/ _x_5 _x_6) (/ _y_5 _y_6) (/ (Variables|Default|GetWallThickness) (.Z (Math|Vector|BreakVector (Variables|Default|GetSizeReference))))))
      (Transformation|SetRelativeLocation _elevator_floor (Math|Vector|MakeVector 0.0 0.0 (* (/ _z_5 2.0) -1.0)) false false))
    (:then_3
      (Transformation|SetRelativeScale3D _elevator_ceiling (Math|Vector|MakeVector (/ _x_7 _x_8) (/ _y_7 _y_8) (/ (Variables|Default|GetWallThickness) (.Z (Math|Vector|BreakVector (Variables|Default|GetSizeReference))))))
      (Transformation|SetRelativeLocation _elevator_ceiling (Math|Vector|MakeVector 0.0 0.0 (/ _z_6 2.0)) false false))
    (:then_4
      (Transformation|SetRelativeScale3D _elevator_backwall (Math|Vector|MakeVector (/ _x _x_9) (/ (Variables|Default|GetWallThickness) (.Y (Math|Vector|BreakVector (Variables|Default|GetSizeReference)))) (/ _z _z_7)))
      (Transformation|SetRelativeLocation _elevator_backwall (Math|Vector|MakeVector 0.0 (* (/ _y 2.0) -1.0) 0.0) false false))))

(fn LinkingtoElevatorButtonsinEachFloor
  (bind _linkingbuttonsineachfloor (Variables|Default|GetLinkingButtonsInEachFloor))
  (if (> (Utilities|Map|Length _linkingbuttonsineachfloor) 0)
    (bind _keys (Utilities|Map|Keys _linkingbuttonsineachfloor))
    (for _array_element _keys
      (LocalVariables|SetFloorIndex _array_element)
      (LocalVariables|SetElevatorCaller (.Value (Utilities|Map|Find (Variables|Default|GetLinkingButtonsInEachFloor) (LocalVariables|GetFloorIndex))))
      (Utilities|Map|Add (Variables|Default|GetLinkingTransformOfEachFloors) (LocalVariables|GetFloorIndex) (Variables|/Game/RX_Jonah/ElevatorSystem/BP_ElevatorCaller.BP_ElevatorCaller_C|GetElevatorLinkingTargetTransform (LocalVariables|GetElevatorCaller))))))