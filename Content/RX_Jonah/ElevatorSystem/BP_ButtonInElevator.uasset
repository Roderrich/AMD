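; Interactable floor button inside an elevator that a player activates to select a destination floor.
; It labels itself from its floor number, showing G for 0 and Top for 999, and builds a matching crosshair prompt.
; Collision overlap stores the Player_RebelX as passenger, and activation calls OnButtonInElevatorPressed with floor, linking transform and passenger.
; Other interaction queries are stubs.
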(event OnComponentBeginOverlap(Collision_Button)
  (params (OverlappedComponent :type Primitive%20Component%20Object%20Reference) (OtherActor :type Actor%20Object%20Reference) (OtherComp :type Primitive%20Component%20Object%20Reference) (OtherBodyIndex :type Integer) (bFromSweep :type Boolean) (SweepResult :type Hit%20Result%20Structure%20%28by%20ref%29))
  (bind _asplayer_rebel_x (Utilities|Casting|CastToPlayer_RebelX OtherActor))
  (Variables|Default|SetElevatorPassenger _asplayer_rebel_x)
  (Development|PrintString "Player Overlap Button In Elevator"))

(event EventBeginPlay
  (CallFunction|UpdateButtonAppearence))

(event Collision|EventActorBeginOverlap
  (params (OtherActor :type Actor%20Object%20Reference)))

(event EventTick
  (params (DeltaSeconds :type Float%20%28single-precision%29)))

(event EventActivateSceneObject
  (Default|CallOnButtoninElevatorPressed (Variables|Default|GetFloorNum) (Variables|Default|GetLinkingTransform) (Variables|Default|GetElevatorPassenger)))

(event EventAttemptConsumeInteractable)

(fn ConstructionScript)

(fn UpdateButtonAppearence
  (bind _floornum (Variables|Default|GetFloorNum))
  (bind _returnvalue (Utilities|Text|ToText(Integer) _floornum))
  (Rendering|Components|TextRender|SetText (Variables|Default|GetText_Floor) (select (Utilities|Enum|Equal(Enum) _returnvalue (Utilities|Text|MakeLiteralText "0")) (Utilities|Text|MakeLiteralText "G") (select (Utilities|Enum|Equal(Enum) _returnvalue (Utilities|Text|MakeLiteralText "999")) (Utilities|Text|MakeLiteralText "Top") _returnvalue))))

(fn GetAmmoInfo
  (return false "NewEnumerator0"))

(fn GetCrosshairPrompt
  (bind _floornum (Variables|Default|GetFloorNum))
  (Variables|Default|SetInteraction%20Message (Utilities|Text|ToText(String) (Utilities|String|Append "Press ButtonTo " (select (== _floornum 0) "G" (Utilities|String|SelectString "Top" (Utilities|String|ToString(Integer) _floornum) (== _floornum 999))) " Floor")))
  (return (Variables|Default|GetInteraction%20Message) "E"))

(fn GetHealthInfo
  (return false 0.0))

(fn GetInteractionType
  (return false "NewEnumerator2"))

(fn GetIsConsumeable
  (return false))

(fn GetSceneInfo
  (return false))