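; Elevator call button that, when activated as a scene object and flagged as working, brings its linked elevator to a stored target transform.
; CallElevator skips elevators already there, otherwise a timeline lerps from the elevator's current transform to the target each update.
; The construction script tints the button by working state, and interaction getters supply an "E" crosshair prompt.
; The box-overlap timer for debug hover traces is disconnected, leaving begin overlap empty.
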(event OnComponentBeginOverlap(Box)
  (params (OverlappedComponent :type Primitive%20Component%20Object%20Reference) (OtherActor :type Actor%20Object%20Reference) (OtherComp :type Primitive%20Component%20Object%20Reference) (OtherBodyIndex :type Integer) (bFromSweep :type Boolean) (SweepResult :type Hit%20Result%20Structure%20%28by%20ref%29)))

(event OnComponentEndOverlap(Box)
  (params (OverlappedComponent :type Primitive%20Component%20Object%20Reference) (OtherActor :type Actor%20Object%20Reference) (OtherComp :type Primitive%20Component%20Object%20Reference) (OtherBodyIndex :type Integer))
  (Utilities|Casting|CastToPlayer_RebelX OtherActor)
  (Variables|Default|SetPlayerPawn 0)
  (Utilities|Time|ClearandInvalidateTimerbyHandle (Variables|Default|GetCheckIsHoveredElevatorButtonTimer)))

(event Custom|CheckIsMouseHoveredOnElevatorButton
  (bind _playerpawn (Variables|Default|GetPlayerPawn))
  (bind _camera_view (Variables|/Game/RebelX_Core/Blueprints/Player_RebelX.Player_RebelX_C|GetCamera%20View _playerpawn))
  (bind _returnvalue (Transformation|GetWorldLocation _camera_view))
  (bind (_outhit _returnvalue_2) (Collision|LineTraceByChannel _returnvalue (+ _returnvalue (* (Math|Vector|GetForwardVector _camera_view) 5e+03)) "TraceTypeQuery3" true 0 "ForDuration"))
  (Development|PrintString (Utilities|String|Append "Is Hit?" (Utilities|String|ToString(Boolean) _returnvalue_2) (Utilities|GetDisplayName (.HitActor (Collision|BreakHitResult _outhit))) (Utilities|GetDisplayName (.HitComponent (Collision|BreakHitResult _outhit))))))

(event Custom|CallElevator
  (bind _elevatorlinkingtargettransform (Variables|Default|GetElevatorLinkingTargetTransform))
  (bind _linkingelevator (Variables|Default|GetLinkingElevator))
  (bind (_location _rotation) (Math|Transform|BreakTransform _elevatorlinkingtargettransform))
  (bind _defaultsceneroot (Variables|/Game/RX_Jonah/ElevatorSystem/BP_EditableElevator.BP_EditableElevator_C|GetDefaultSceneRoot _linkingelevator))
  (if (or (Utilities|Operators|NotEqual(!=) (Transformation|GetWorldLocation _defaultsceneroot) _location 0.0) (Utilities|Operators|NotEqual(!=) (Transformation|GetWorldRotation _defaultsceneroot) _rotation 0.0))
    (Development|PrintString "ElevatorCome!!!!!")
    (bind _movement (Timeline|Timeline_MoveElevator PlayFromStart)
      (:Update
        (Transformation|SetActorTransform (Variables|Default|GetLinkingElevator) (Math|Transform|Lerp(Transform) (Transformation|GetActorTransform (Variables|Default|GetLinkingElevator)) (Variables|Default|GetElevatorLinkingTargetTransform) _movement)))
      (:Finished
        (Development|PrintString "ElevatorMoveToTargetPlace!!!!!")))))

(event EventActivateSceneObject
  (if (Variables|Default|GetIsButtonWorked)
    (CallFunction|CallElevator)))

(fn ConstructionScript
  (bind _returnvalue (Rendering|Material|CreateDynamicMaterialInstance (Variables|Default|GetCylinder_ElevatorButton) 0 "/Game/RX_Jonah/ElevatorSystem/MI_ElevatorCaller.MI_ElevatorCaller" "None" :!class /Script/Engine.PrimitiveComponent))
  (Rendering|Material|SetVectorParameterValue _returnvalue "Color" (select (Variables|Default|GetIsButtonWorked) "(R=0.000000,G=1.000000,B=0.666667,A=1.000000)" "(R=1.000000,G=0.033333,B=0.000000,A=1.000000)") :!class /Script/Engine.MaterialInstanceDynamic))

(fn GetAmmoInfo
  (return false "NewEnumerator0"))

(fn GetCrosshairPrompt
  (return (Variables|Default|GetInteractionMessage) "E"))

(fn GetHealthInfo
  (return false 0.0))

(fn GetInteractionType
  (return false "NewEnumerator2"))

(fn GetIsConsumeable
  (return false))

(fn GetSceneInfo
  (return false))