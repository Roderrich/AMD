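; In-cabin elevator control panel that carries a passenger to a chosen floor.
; On BeginPlay it spawns and attaches a row of floor buttons from FloorWithTransform, spaced using the linked elevator's size.
; A press attaches the passenger to the elevator, then a timeline disables their movement and lerps the elevator from its current transform to the target.
; On finish it restores walking and input, then fires the arrival dispatcher.
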(event Custom|MoveElevatorWithPlayer
  (params (TargetFloor :type Integer) (TargetTransform :type Transform) (Passenger :type Player%20Rebel%20X%20Object%20Reference))
  (bind (_location _rotation) (Math|Transform|BreakTransform TargetTransform))
  (bind _linkingelevator (Variables|Default|GetLinkingElevator))
  (bind _charactermovement (Variables|/Script/Engine.Character|GetCharacterMovement Passenger))
  (bind _returnvalue (Transformation|GetActorTransform _linkingelevator))
  (bind (_location_2 _rotation_2) (Math|Transform|BreakTransform _returnvalue))
  (if (or (Utilities|Operators|NotEqual(!=) _location_2 _location 0.0) (Utilities|Operators|NotEqual(!=) _rotation_2 _rotation 0.0))
    (bind _movement (Timeline|Timeline PlayFromStart)
      (:Update
        (Pawn|Components|CharacterMovement|DisableMovement _charactermovement)
        (Transformation|SetActorTransform (Variables|Default|GetLinkingElevator) (Math|Transform|MakeTransform (.Location (Math|Transform|BreakTransform (Math|Transform|Lerp(Transform) (Transformation|GetActorTransform (Variables|Default|GetLinkingElevator)) TargetTransform _movement))) (.Rotation (Math|Transform|BreakTransform (Math|Transform|Lerp(Transform) (Transformation|GetActorTransform (Variables|Default|GetLinkingElevator)) TargetTransform _movement))) (.Scale (Math|Transform|BreakTransform (Math|Transform|Lerp(Transform) (Transformation|GetActorTransform (Variables|Default|GetLinkingElevator)) TargetTransform _movement))))))
      (:Finished
        (Input|SetIgnoreMoveInput (Game|GetPlayerController 0) false)
        (Pawn|Components|CharacterMovement|SetMovementMode _charactermovement "MOVE_Walking" 0)
        (Default|CallOnElevatorTakePassengertoTargetFloor Passenger TargetTransform TargetFloor)))))

(event EventBeginPlay
  (CallFunction|UpdateControllerAppearance))

(event Collision|EventActorBeginOverlap
  (params (OtherActor :type Actor%20Object%20Reference)))

(event EventTick
  (params (DeltaSeconds :type Float%20%28single-precision%29)))

(fn ConstructionScript)

(fn UpdateControllerAppearance
  (bind _floorwithtransform (Variables|Default|GetFloorWithTransform))
  (if (> (Utilities|Map|Length _floorwithtransform) 0)
    (bind _keys (Utilities|Map|Keys _floorwithtransform))
    (for (_array_element _array_index) _keys
      (LocalVariables|SetCurrentFloor _array_element)
      (bind _returnvalue (Game|SpawnActorfromClass "/Game/RX_Jonah/ElevatorSystem/BP_ButtonInElevator.BP_ButtonInElevator_C" (Math|Transform|MakeTransform "0, 0, 0" "0, 0, 0" "1.000000,1.000000,1.000000") "Undefined" "MultiplyWithRoot" 0 (LocalVariables|GetCurrentFloor) (.Value (Utilities|Map|Find (Variables|Default|GetFloorWithTransform) (LocalVariables|GetCurrentFloor))) 0))
      (bind _output_get (LocalVariables|SetButtonInElevator _returnvalue))
      (EventDispatchers|BindEventtoOnButtoninElevatorPressed _output_get (EventDispatchers|CreateEvent :!event OnButtoninElevatorPressed))
      (Transformation|AttachActorToActor _output_get self "None" "SnapToTarget" "SnapToTarget" "SnapToTarget" true)
      (Transformation|SetRelativeTransform (Variables|/Game/RX_Jonah/ElevatorSystem/BP_ButtonInElevator.BP_ButtonInElevator_C|GetDefaultSceneRoot (LocalVariables|GetButtonInElevator)) (CallFunction|GetButtonTransformBasedonFloor (Utilities|Map|Length (Variables|Default|GetFloorWithTransform)) _array_index) false false)
      (Utilities|Map|Add (Variables|Default|GetFloorWithButtons) (LocalVariables|GetCurrentFloor) (LocalVariables|GetButtonInElevator)))))

(fn GetButtonTransformBasedonFloor
  (params (ButtonsTotalNum :type Integer) (Floor :type Integer))
  (bind _returnvalue (Math|Transform|MakeTransform "0, 0, 0"))
  (bind _controllertransformoffset (Variables|Default|GetControllerTransformOffset))
  (bind (_location _rotation _scale) (Math|Transform|BreakTransform _returnvalue))
  (bind (_location_2 _rotation_2) (Math|Transform|BreakTransform _controllertransformoffset))
  (bind _returnvalue_2 (+ _location _location_2))
  (bind (_x _y _z) (Math|Vector|BreakVector _returnvalue_2))
  (return (Math|Transform|MakeTransform (Math|Vector|MakeVector (+ _x (/ (.X (Math|Vector|BreakVector (Variables|/Game/RX_Jonah/ElevatorSystem/BP_EditableElevator.BP_EditableElevator_C|GetElevatorSize (Variables|Default|GetLinkingElevator)))) 2.0)) (+ (- _y (* ButtonsTotalNum (Variables|Default|GetDistanceBetweenEachButton) 0.5)) (* Floor (Variables|Default|GetDistanceBetweenEachButton))) (+ _z (* (/ (.Z (Math|Vector|BreakVector (Variables|/Game/RX_Jonah/ElevatorSystem/BP_EditableElevator.BP_EditableElevator_C|GetElevatorSize (Variables|Default|GetLinkingElevator)))) 2.0) -1.0) (Variables|Default|GetDistanceFromTheBottomFloor))) (Math|Rotator|CombineRotators _rotation _rotation_2) _scale)))

(fn OnButtoninElevatorPressed
  (params (ButtonFloor :type Integer) (FloorTransform :type Transform) (Passenger :type Player%20Rebel%20X%20Object%20Reference))
  (Utilities|IsValid Passenger
    (:Is%20Valid
      (Transformation|AttachActorToActor Passenger (Variables|Default|GetLinkingElevator) "None" "SnapToTarget" "SnapToTarget" "SnapToTarget" true)
      (CallFunction|MoveElevatorwithPlayer ButtonFloor FloorTransform Passenger))))