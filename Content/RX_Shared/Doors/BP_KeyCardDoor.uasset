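; BP_KeyCardDoor is a door that unlocks when the player enters its box carrying the required key card.
; The overlap checks the player's backpack key cards by IDNeeded and clears Locked.
; Interaction-interface functions supply a locked or unlocked crosshair prompt, but ActivateSceneObject does nothing.
; Door-opening timelines, movement nodes and timers for auto-close and an upward player teleport are disconnected, so unlocking moves nothing.
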(event OnComponentBeginOverlap(Box)
  (params (OverlappedComponent :type Primitive%20Component%20Object%20Reference) (OtherActor :type Actor%20Object%20Reference) (OtherComp :type Primitive%20Component%20Object%20Reference) (OtherBodyIndex :type Integer) (bFromSweep :type Boolean) (SweepResult :type Hit%20Result%20Structure%20%28by%20ref%29))
  (bind _asplayer_rebel_x (Utilities|Casting|CastToPlayer_RebelX OtherActor))
  (if (Utilities|Array|Get(acopy) (Variables|/Game/RX_Roderrich/BPC_Backpack.BPC_Backpack_C|GetKeyCards (Variables|/Game/RebelX_Core/Blueprints/Player_RebelX.Player_RebelX_C|GetBPC_Backpack _asplayer_rebel_x)) (Variables|Default|GetID%20Needed))
    (CallFunction|ClearanceAquirred)))

(event Custom|ClearanceAquirred
  (Variables|Default|SetLocked false))

(event Custom|Close%20Door
  (bind _newtrack_0 (Timeline|Timeline_2 ReverseFromEnd)
    (:Finished
      (bind _newtrack_0_2 (Timeline|Timeline_1 ReverseFromEnd)))))

(event Custom|Teleport
  (bind _as_player_rebel_x (Variables|Default|GetAs%20Player%20Rebel%20X))
  (if (Variables|Default|GetReady%20To%20Tp)
    (Transformation|SetActorLocation _as_player_rebel_x (+ (Transformation|GetActorLocation _as_player_rebel_x) "0.000000,0.000000,451.000000") false false)))

(event EventBeginPlay
  (bind _asplayer_rebel_x (Utilities|Casting|CastToPlayer_RebelX (Game|GetPlayerCharacter 0)))
  (Variables|Default|SetAs%20Player%20Rebel%20X _asplayer_rebel_x))

(event Collision|EventActorBeginOverlap
  (params (OtherActor :type Actor%20Object%20Reference)))

(event EventTick
  (params (DeltaSeconds :type Float%20%28single-precision%29)))

(event EventActivateSceneObject
  (if (Variables|Default|GetLocked)
    _))

(fn ConstructionScript)

(fn GetAmmoInfo
  (return false "NewEnumerator0"))

(fn GetCrosshairPrompt
  (if (Variables|Default|GetLocked)
    (return (Variables|Default|GetLocked%20Message) "[E]")
    (else
      (return (Variables|Default|GetUnlocked%20Message) ""))))

(fn GetHealthInfo
  (return false 0.0))

(fn GetInteractionType
  (return false "NewEnumerator2"))

(fn GetIsConsumeable
  (return false))

(fn GetSceneInfo
  (return false))