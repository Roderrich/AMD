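; BP_KCDoor is a door actor that swings open once when its OpenDoor event is called with a yaw offset.
; BeginPlay caches the actor's starting rotation as the closed pose.
; OpenDoor runs through a DoOnce into a Timeline that lerps relative rotation from the cached pose to the offset yaw, with pitch and roll zeroed.
; No closing or reset logic is present, and overlap and tick are unused.
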(event EventBeginPlay
  (Variables|Default|SetRotate (Transformation|GetActorRotation)))

(event Collision|EventActorBeginOverlap
  (params (OtherActor :type Actor%20Object%20Reference)))

(event EventTick
  (params (DeltaSeconds :type Float%20%28single-precision%29)))

(event EventOpenDoor
  (params (Rotation :type Float%20%28double-precision%29))
  (bind _rotate (Variables|Default|GetRotate))
  (Utilities|FlowControl|DoOnce false
    (:Completed
      (bind _newtrack_0 (Timeline|Timeline PlayFromStart)
        (:Update
          (Transformation|SetActorRelativeRotation (Math|Rotator|Lerp(Rotator) _rotate (Math|Rotator|MakeRotator 0.0 0.0 (+ (.Yaw (Math|Rotator|BreakRotator _rotate)) Rotation)) _newtrack_0)))))))

(fn ConstructionScript)