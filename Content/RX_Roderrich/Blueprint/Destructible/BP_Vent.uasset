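; Destructible vent actor that is removed when the player damages it.
; AnyDamage compares the damage causer's class display name to a hard-coded Player_RebelX_C string, then prints it and destroys the actor.
; Getter functions supply a "Pry Open Vent" crosshair prompt with a [Q] tooltip and return false or default values for ammo, health, interaction, consumable and scene queries.
; No pry input is handled here.
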(event EventBeginPlay)

(event Collision|EventActorBeginOverlap
  (params (OtherActor :type Actor%20Object%20Reference)))

(event EventTick
  (params (DeltaSeconds :type Float%20%28single-precision%29)))

(event Game|Damage|EventAnyDamage
  (params (Damage :type Float%20%28single-precision%29) (DamageType :type Damage%20Type%20Object%20Reference) (InstigatedBy :type Controller%20Object%20Reference) (DamageCauser :type Actor%20Object%20Reference))
  (bind _returnvalue (Utilities|GetClass DamageCauser))
  (bind _returnvalue_2 (Utilities|GetClassDisplayName _returnvalue))
  (if (Utilities|Enum|Equal(Enum) _returnvalue_2 "Player_RebelX_C")
    (Development|PrintString _returnvalue_2)
    (Actor|DestroyActor)))

(fn ConstructionScript)

(fn GetAmmoInfo
  (return false "NewEnumerator0"))

(fn GetCrosshairPrompt
  (return "Pry Open Vent" "Press [Q] to Pry"))

(fn GetHealthInfo
  (return false 0.0))

(fn GetInteractionType
  (return false "NewEnumerator4"))

(fn GetIsConsumeable
  (return false))

(fn GetSceneInfo
  (return false))