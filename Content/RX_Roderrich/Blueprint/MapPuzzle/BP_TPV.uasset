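; BP_TPV is an interactable vent that teleports the player to a Target when activated.
; It answers interaction queries with an "Enter Vent" prompt.
; Activation plays the GM_RebelX widget's vent message forward and uses its returned time to delay the teleport.
; The player character then takes the Target root's transform, nudged along its forward vector, and the message plays in reverse.
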(event Custom|Teleport
  (bind _target (Variables|Default|GetTarget))
  (bind _rootcomponent (Variables|/Script/Engine.Actor|GetRootComponent _target))
  (bind _returnvalue (Transformation|GetWorldTransform _rootcomponent))
  (Transformation|SetActorTransform (Game|GetPlayerCharacter 0) (Math|Transform|MakeTransform (+ (.location _returnvalue) (* (Math|Vector|GetForwardVector _rootcomponent) 5e+01)) (.rotation _returnvalue) (.scale _returnvalue)))
  (Class|BPIWidget|EnterVent(Message) (Variables|/Game/RebelX_Core/Blueprints/GM_RebelX.GM_RebelX_C|GetWidget (Variables|Default|GetAs%20GM%20Rebel%20X)) "Reverse"))

(event EventBeginPlay
  (bind _asgm_rebel_x (Utilities|Casting|CastToGM_RebelX (Game|GetGameMode)))
  (Variables|Default|SetAs%20GM%20Rebel%20X _asgm_rebel_x))

(event Collision|EventActorBeginOverlap
  (params (OtherActor :type Actor%20Object%20Reference)))

(event EventTick
  (params (DeltaSeconds :type Float%20%28single-precision%29)))

(event EventActivateSceneObject
  (bind _time (Class|BPIWidget|EnterVent(Message) (Variables|/Game/RebelX_Core/Blueprints/GM_RebelX.GM_RebelX_C|GetWidget (Variables|Default|GetAs%20GM%20Rebel%20X)) "Forward"))
  (Utilities|Time|SetTimerbyEvent (delegate Custom|Teleport) _time))

(fn ConstructionScript)

(fn GetAmmoInfo
  (return false "NewEnumerator0"))

(fn GetCrosshairPrompt
  (return "Enter Vent" "Press [E] to Enter"))

(fn GetHealthInfo
  (return false 0.0))

(fn GetInteractionType
  (return false "NewEnumerator2"))

(fn GetIsConsumeable
  (return false))

(fn GetSceneInfo
  (return false))