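; BP_Vent is a map vent that teleports any actor entering its Box trigger to the transform of a linked OutActor.
; On overlap it calls EnterVentMessage forward on the GM_RebelX game mode's widget and uses the returned value as a timer delay.
; When the timer fires, Teleport moves the overlapping actor without sweep, then calls EnterVentMessage in reverse.
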(event OnComponentBeginOverlap(Box)
  (params (OverlappedComponent :type Primitive%20Component%20Object%20Reference) (OtherActor :type Actor%20Object%20Reference) (OtherComp :type Primitive%20Component%20Object%20Reference) (OtherBodyIndex :type Integer) (bFromSweep :type Boolean) (SweepResult :type Hit%20Result%20Structure%20%28by%20ref%29))
  (bind _time (Class|BPIWidget|EnterVent(Message) (Variables|/Game/RebelX_Core/Blueprints/GM_RebelX.GM_RebelX_C|GetWidget (Variables|Default|GetAs%20GM%20Rebel%20X)) "Forward"))
  (Utilities|Time|SetTimerbyEvent (delegate Custom|Teleport) _time))

(event Custom|CustomEvent)

(event Custom|Teleport
  (Transformation|SetActorTransform (stale OnComponentBeginOverlap(Box) OtherActor) (Transformation|GetWorldTransform (Variables|/Script/Engine.Actor|GetRootComponent (Variables|Default|GetOutActor))))
  (Class|BPIWidget|EnterVent(Message) (Variables|/Game/RebelX_Core/Blueprints/GM_RebelX.GM_RebelX_C|GetWidget (Variables|Default|GetAs%20GM%20Rebel%20X)) "Reverse"))

(event EventBeginPlay
  (bind _asgm_rebel_x (Utilities|Casting|CastToGM_RebelX (Game|GetGameMode)))
  (Variables|Default|SetAs%20GM%20Rebel%20X _asgm_rebel_x))

(event Collision|EventActorBeginOverlap
  (params (OtherActor :type Actor%20Object%20Reference)))

(event EventTick
  (params (DeltaSeconds :type Float%20%28single-precision%29)))

(fn ConstructionScript)