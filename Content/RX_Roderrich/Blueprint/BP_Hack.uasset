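; BP_Hack is an interactable hack objective that offers a crosshair prompt and starts a timed hack when activated.
; Activation runs once until reset, starts the hack on the GM_RebelX widget, triggers an encounter message and broadcasts HackStarted.
; AI soldiers overlapping component R toggle the widget's disrupted state.
; When the widget reports completion, it clears the prompt and tooltip and broadcasts HackFinished.
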(event OnComponentBeginOverlap(r)
  (params (OverlappedComponent :type Primitive%20Component%20Object%20Reference) (OtherActor :type Actor%20Object%20Reference) (OtherComp :type Primitive%20Component%20Object%20Reference) (OtherBodyIndex :type Integer) (bFromSweep :type Boolean) (SweepResult :type Hit%20Result%20Structure%20%28by%20ref%29))
  (Utilities|Casting|CastToAI_Soldier_Child OtherActor)
  (Default|DisruptedEvent (Variables|/Game/RebelX_Core/Blueprints/GM_RebelX.GM_RebelX_C|GetWidget (Variables|Default|GetAs%20GM%20Rebel%20X)) true))

(event OnComponentEndOverlap(r)
  (params (OverlappedComponent :type Primitive%20Component%20Object%20Reference) (OtherActor :type Actor%20Object%20Reference) (OtherComp :type Primitive%20Component%20Object%20Reference) (OtherBodyIndex :type Integer))
  (Utilities|Casting|CastToAI_Soldier_Child OtherActor)
  (Default|DisruptedEvent (Variables|/Game/RebelX_Core/Blueprints/GM_RebelX.GM_RebelX_C|GetWidget (Variables|Default|GetAs%20GM%20Rebel%20X)) false))

(event Custom|CustomEvent
  (Utilities|FlowControl|DoOnce false) ; enters at Reset
)

(event Custom|HackFinished_Event
  (Variables|Default|SetPrompt "")
  (Variables|Default|SetTooltip "")
  (Default|CallHackFinished))

(event EventBeginPlay)

(event Collision|EventActorBeginOverlap
  (params (OtherActor :type Actor%20Object%20Reference)))

(event EventTick
  (params (DeltaSeconds :type Float%20%28single-precision%29)))

(event EventActivateSceneObject
  (Utilities|FlowControl|DoOnce false
    (:Completed
      (bind _asgm_rebel_x (Utilities|Casting|CastToGM_RebelX (Game|GetGameMode)))
      (bind _output_get (Variables|Default|SetAs%20GM%20Rebel%20X _asgm_rebel_x))
      (Default|HackEvent (Variables|/Game/RebelX_Core/Blueprints/GM_RebelX.GM_RebelX_C|GetWidget _output_get) (Variables|Default|GetTime))
      (Class|BPIEncounterManager|ActivateEncounter(Message) (Variables|Default|GetActor))
      (Default|CallHackStarted)
      (EventDispatchers|AssignHackFinished (Variables|/Game/RebelX_Core/Blueprints/GM_RebelX.GM_RebelX_C|GetWidget _output_get) (delegate Custom|HackFinished_Event)))))

(fn ConstructionScript)

(fn GetAmmoInfo
  (return false "NewEnumerator0"))

(fn GetCrosshairPrompt
  (return (Variables|Default|GetPrompt) (Variables|Default|GetTooltip)))

(fn GetHealthInfo
  (return false 0.0))

(fn GetInteractionType
  (return false "NewEnumerator2"))

(fn GetIsConsumeable
  (return false))

(fn GetSceneInfo
  (return false))