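; BP_Lights is a configurable building light prop with a selectable mesh, emissive strength and colour.
; The construction script applies MI_LIGHTASSETS to one static mesh component, then sets its LightStrength and Colour material parameters from the matching variables.
; The Selection value swaps between four light meshes, whose numbers do not match the option names.
; All logic runs at construction, as the event graph is empty.
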(event EventBeginPlay)

(event Collision|EventActorBeginOverlap
  (params (OtherActor :type Actor%20Object%20Reference)))

(event EventTick
  (params (DeltaSeconds :type Float%20%28single-precision%29)))

(fn ConstructionScript
  (bind _sm_bld_light_12 (Variables|Default|GetSM_Bld_Light_12))
  (bind _sm_bld_light_12_2 (Variables|Default|GetSM_Bld_Light_12))
  (Rendering|Material|SetMaterial _sm_bld_light_12 0 "/Game/RX_Roderrich/Materials/Lights/MI_LIGHTASSETS.MI_LIGHTASSETS")
  (Rendering|Material|SetScalarParameterValueonMaterials _sm_bld_light_12 "LightStrength" (Variables|Default|GetLightStrength))
  (Rendering|Material|SetVectorParameterValueonMaterials _sm_bld_light_12 "Colour" (Math|Conversions|ToVector(LinearColor) (Variables|Default|GetColour)))
  (switch Utilities|FlowControl|Switch|SwitchonEnum_Lights (Variables|Default|GetSelection)
    (:NewEnumerator0
      (Components|StaticMesh|SetStaticMesh _sm_bld_light_12_2 "/Game/PolygonScifiWorlds/Meshes/Buildings/SM_Bld_Light_03.SM_Bld_Light_03"))
    (:NewEnumerator4
      (Components|StaticMesh|SetStaticMesh _sm_bld_light_12_2 "/Game/PolygonScifiWorlds/Meshes/Buildings/SM_Bld_Light_10.SM_Bld_Light_10"))
    (:NewEnumerator5
      (Components|StaticMesh|SetStaticMesh _sm_bld_light_12_2 "/Game/PolygonScifiWorlds/Meshes/Buildings/SM_Bld_Light_12.SM_Bld_Light_12"))
    (:NewEnumerator6
      (Components|StaticMesh|SetStaticMesh _sm_bld_light_12_2 "/Game/PolygonScifiWorlds/Meshes/Buildings/SM_Bld_Light_06.SM_Bld_Light_06"))))