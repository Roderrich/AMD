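; Keycard-gated interactable elevator that fakes travel by moving the player straight up.
; Overlapping Box with the first backpack keycard flag set unlocks it and changes the crosshair prompt.
; Activation runs chained timelines to slide two door meshes open in stages, then timers and reversed timelines close them.
; After closing and a short delay, a player still inside Box1 is offset upward by a fixed height.
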(event OnComponentBeginOverlap(Box)
  (params (OverlappedComponent :type Primitive%20Component%20Object%20Reference) (OtherActor :type Actor%20Object%20Reference) (OtherComp :type Primitive%20Component%20Object%20Reference) (OtherBodyIndex :type Integer) (bFromSweep :type Boolean) (SweepResult :type Hit%20Result%20Structure%20%28by%20ref%29))
  (bind _asplayer_rebel_x (Utilities|Casting|CastToPlayer_RebelX OtherActor))
  (bind _asbp_backpack (Utilities|Casting|CastToBP_Backpack (Variables|/Game/RebelX_Core/Blueprints/Player_RebelX.Player_RebelX_C|GetVariable_Backpack _asplayer_rebel_x)))
  (if (Utilities|Array|Get(acopy) (Variables|/Game/RX_C_Bailey_Content/Blueprints/BP_Backpack.BP_Backpack_C|GetKeycard%20IDs _asbp_backpack))
    (CallFunction|ClearanceAquirred)))

(event OnComponentBeginOverlap(Box1)
  (params (OverlappedComponent :type Primitive%20Component%20Object%20Reference) (OtherActor :type Actor%20Object%20Reference) (OtherComp :type Primitive%20Component%20Object%20Reference) (OtherBodyIndex :type Integer) (bFromSweep :type Boolean) (SweepResult :type Hit%20Result%20Structure%20%28by%20ref%29))
  (Utilities|Casting|CastToPlayer_RebelX OtherActor)
  (Variables|Default|SetReady%20To%20Tp true))

(event OnComponentEndOverlap(Box1)
  (params (OverlappedComponent :type Primitive%20Component%20Object%20Reference) (OtherActor :type Actor%20Object%20Reference) (OtherComp :type Primitive%20Component%20Object%20Reference) (OtherBodyIndex :type Integer))
  (Utilities|Casting|CastToPlayer_RebelX OtherActor)
  (Variables|Default|SetReady%20To%20Tp false))

(event Custom|ClearanceAquirred
  (Variables|Default|SetUnlocked true)
  (Variables|Default|SetPrompt "Call Elevator"))

(event Custom|Close%20Door
  (bind _cube1 (Variables|Default|GetCube1))
  (bind _cube1_2 (Variables|Default|GetCube1))
  (bind _relativelocation (Variables|/Script/Engine.SceneComponent|GetRelativeLocation _cube1))
  (bind _relativelocation_2 (Variables|/Script/Engine.SceneComponent|GetRelativeLocation _cube1_2))
  (bind _newtrack_0 (Timeline|Timeline_2 ReverseFromEnd)
    (:Update
      (Transformation|SetRelativeLocation _cube1_2 (Math|Vector|MakeVector (.x _relativelocation_2) _newtrack_0 (.z _relativelocation_2)) false false))
    (:Finished
      (bind _newtrack_0_2 (Timeline|Timeline_1 ReverseFromEnd)
        (:Update
          (Transformation|SetRelativeLocation _cube1 (Math|Vector|MakeVector (.x _relativelocation) _newtrack_0_2 (.z _relativelocation)) false false))
        (:Finished
          (Utilities|Time|SetTimerbyEvent (delegate Custom|Teleport) 2.0))))))

(event Custom|Teleport
  (bind _as_player_rebel_x (Variables|Default|GetAs%20Player%20Rebel%20X))
  (if (Variables|Default|GetReady%20To%20Tp)
    (Transformation|SetActorLocation _as_player_rebel_x (+ (Transformation|GetActorLocation _as_player_rebel_x) "0.000000,0.000000,451.000000") false false)))

(event EventBeginPlay
  (bind _asplayer_rebel_x (Utilities|Casting|CastToPlayer_RebelX (Game|GetPlayerCharacter 0)))
  (Variables|Default|SetAs%20Player%20Rebel%20X _asplayer_rebel_x))

(event Collision|EventActorBeginOverlap
  (params (OtherActor :type Actor%20Object%20Reference)))

(event EventTick
  (params (DeltaSeconds :type Float%20%28single-precision%29)))

(event EventActivateSceneObject
  (bind _cube1 (Variables|Default|GetCube1))
  (bind _cube1_2 (Variables|Default|GetCube1))
  (bind _relativelocation (Variables|/Script/Engine.SceneComponent|GetRelativeLocation _cube1))
  (bind _relativelocation_2 (Variables|/Script/Engine.SceneComponent|GetRelativeLocation _cube1_2))
  (if (Variables|Default|GetUnlocked)
    (bind _newtrack_0 (Timeline|Timeline PlayFromStart)
      (:Update
        (Transformation|SetRelativeLocation _cube1 (Math|Vector|MakeVector (.x _relativelocation) _newtrack_0 (.z _relativelocation)) false false))
      (:Finished
        (bind _newtrack_0_2 (Timeline|Timeline_0 PlayFromStart)
          (:Update
            (Transformation|SetRelativeLocation _cube1_2 (Math|Vector|MakeVector (.x _relativelocation_2) _newtrack_0_2 (.z _relativelocation_2)) false false))
          (:Finished
            (Utilities|Time|SetTimerbyEvent (delegate Custom|Close%20Door) 3.0)))))))

(fn ConstructionScript)

(fn GetAmmoInfo
  (return false "NewEnumerator0"))

(fn GetCrosshairPrompt
  (return (Variables|Default|GetPrompt) ""))

(fn GetHealthInfo
  (return false 0.0))

(fn GetInteractionType
  (return false "NewEnumerator2"))

(fn GetIsConsumeable
  (return false))

(fn GetSceneInfo
  (return false))