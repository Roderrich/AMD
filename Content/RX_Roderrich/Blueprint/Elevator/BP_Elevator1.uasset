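; BP_Elevator1 is an elevator actor whose two sliding door panels open and close as the player enters and leaves a trigger box.
; Box1 overlaps play chained timelines: Cube1 slides first, then both panels together, reversed to close, with CompletedOpen and CompletedClose gating each direction.
; Keycard clearance and a timed teleport raising the player are present but unwired.
; Interaction info functions return empty defaults.
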(event OnComponentBeginOverlap(Box)
  (params (OverlappedComponent :type Primitive%20Component%20Object%20Reference) (OtherActor :type Actor%20Object%20Reference) (OtherComp :type Primitive%20Component%20Object%20Reference) (OtherBodyIndex :type Integer) (bFromSweep :type Boolean) (SweepResult :type Hit%20Result%20Structure%20%28by%20ref%29)))

(event OnComponentBeginOverlap(Box1)
  (params (OverlappedComponent :type Primitive%20Component%20Object%20Reference) (OtherActor :type Actor%20Object%20Reference) (OtherComp :type Primitive%20Component%20Object%20Reference) (OtherBodyIndex :type Integer) (bFromSweep :type Boolean) (SweepResult :type Hit%20Result%20Structure%20%28by%20ref%29))
  (bind _cube1 (Variables|Default|GetCube1))
  (bind _cube1_2 (Variables|Default|GetCube1))
  (bind _relativelocation (Variables|/Script/Engine.SceneComponent|GetRelativeLocation _cube1))
  (bind _relativelocation_2 (Variables|/Script/Engine.SceneComponent|GetRelativeLocation _cube1_2))
  (Utilities|Casting|CastToPlayer_RebelX OtherActor)
  (if (Variables|Default|GetCompleted%20Close)
    (Variables|Default|SetCompleted%20Close false)
    (bind _newtrack_0 (Timeline|Timeline PlayFromStart)
      (:Update
        (Transformation|SetRelativeLocation _cube1 (Math|Vector|MakeVector (.x _relativelocation) _newtrack_0 (.z _relativelocation)) false false))
      (:Finished
        (bind _newtrack_0_2 (Timeline|Timeline_0 Play)
          (:Update
            (Transformation|SetRelativeLocation _cube1_2 (Math|Vector|MakeVector (.x _relativelocation_2) _newtrack_0_2 (.z _relativelocation_2)) false false))
          (:Finished
            (Variables|Default|SetCompleted%20Open true)))))))

(event OnComponentEndOverlap(Box1)
  (params (OverlappedComponent :type Primitive%20Component%20Object%20Reference) (OtherActor :type Actor%20Object%20Reference) (OtherComp :type Primitive%20Component%20Object%20Reference) (OtherBodyIndex :type Integer))
  (bind _cube1 (Variables|Default|GetCube1))
  (bind _cube1_2 (Variables|Default|GetCube1))
  (bind _relativelocation (Variables|/Script/Engine.SceneComponent|GetRelativeLocation _cube1))
  (bind _relativelocation_2 (Variables|/Script/Engine.SceneComponent|GetRelativeLocation _cube1_2))
  (Utilities|Casting|CastToPlayer_RebelX OtherActor)
  (if (Variables|Default|GetCompleted%20Open)
    (Variables|Default|SetCompleted%20Open false)
    (bind _newtrack_0 (Timeline|Timeline_2 ReverseFromEnd)
      (:Update
        (Transformation|SetRelativeLocation _cube1_2 (Math|Vector|MakeVector (.x _relativelocation_2) _newtrack_0 (.z _relativelocation_2)) false false))
      (:Finished
        (bind _newtrack_0_2 (Timeline|Timeline_1 ReverseFromEnd)
          (:Update
            (Transformation|SetRelativeLocation _cube1 (Math|Vector|MakeVector (.x _relativelocation) _newtrack_0_2 (.z _relativelocation)) false false))
          (:Finished
            (Variables|Default|SetCompleted%20Open false)
            (Variables|Default|SetCompleted%20Close true)))))))

(event Custom|ClearanceAquirred
  (Variables|Default|SetCompleted%20Open true)
  (Variables|Default|SetPrompt "Call Elevator"))

(event Custom|Teleport
  (bind _as_player_rebel_x (Variables|Default|GetAs%20Player%20Rebel%20X))
  (Utilities|FlowControl|DoOnce false
    (:Completed
      (Transformation|SetActorLocation _as_player_rebel_x (+ (Transformation|GetActorLocation _as_player_rebel_x) "0.000000,0.000000,450.000000") false false))))

(event EventBeginPlay
  (bind _asplayer_rebel_x (Utilities|Casting|CastToPlayer_RebelX (Game|GetPlayerCharacter 0)))
  (Variables|Default|SetAs%20Player%20Rebel%20X _asplayer_rebel_x))

(event Collision|EventActorBeginOverlap
  (params (OtherActor :type Actor%20Object%20Reference)))

(event EventTick
  (params (DeltaSeconds :type Float%20%28single-precision%29)))

(fn ConstructionScript)

(fn GetAmmoInfo
  (return false "NewEnumerator0"))

(fn GetCrosshairPrompt
  (return "" ""))

(fn GetHealthInfo
  (return false 0.0))

(fn GetInteractionType
  (return false "NewEnumerator2"))

(fn GetIsConsumeable
  (return false))

(fn GetSceneInfo
  (return false))