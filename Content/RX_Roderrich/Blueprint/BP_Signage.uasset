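; BP_Signage is a sign actor that shows configurable text with optional left and right elements.
; On BeginPlay it sets the TextRender to the Value variable.
; The Left and Right booleans then reveal Cube1 and Cube2 respectively.
; The construction script is empty, so the text and cube visibility apply only at runtime.
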(event EventBeginPlay
  (Rendering|Components|TextRender|SetText (Variables|Default|GetTextRender) (Variables|Default|GetValue))
  (Utilities|FlowControl|Sequence
    (:then_0
      (if (Variables|Default|GetLeft)
        (Rendering|SetVisibility (Variables|Default|GetCube1) true false)))
    (:then_1
      (if (Variables|Default|GetRight)
        (Rendering|SetVisibility (Variables|Default|GetCube2) true false)))))

(event Collision|EventActorBeginOverlap
  (params (OtherActor :type Actor%20Object%20Reference)))

(event EventTick
  (params (DeltaSeconds :type Float%20%28single-precision%29)))

(fn ConstructionScript)