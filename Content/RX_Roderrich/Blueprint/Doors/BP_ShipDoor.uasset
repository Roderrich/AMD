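; BP_ShipDoor is a two-panel sliding ship door that opens while the Player_RebelX character is inside its trigger box.
; BeginPlay applies a configurable world scale to the box.
; Overlap begin plays two timelines that drive the relative X of Cube1 and Cube2, leaving Y and Z unchanged.
; Overlap end reverses both timelines to close the door.
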(event OnComponentBeginOverlap(Box)
  (params (OverlappedComponent :type Primitive%20Component%20Object%20Reference) (OtherActor :type Actor%20Object%20Reference) (OtherComp :type Primitive%20Component%20Object%20Reference) (OtherBodyIndex :type Integer) (bFromSweep :type Boolean) (SweepResult :type Hit%20Result%20Structure%20%28by%20ref%29))
  (bind _cube1 (Variables|Default|GetCube1))
  (bind _cube2 (Variables|Default|GetCube2))
  (bind _relativelocation (Variables|/Script/Engine.SceneComponent|GetRelativeLocation _cube1))
  (bind _relativelocation_2 (Variables|/Script/Engine.SceneComponent|GetRelativeLocation _cube2))
  (Utilities|Casting|CastToPlayer_RebelX OtherActor)
  (Utilities|FlowControl|Sequence
    (:then_0
      (bind _newtrack_0 (Timeline|Timeline Play)
        (:Update
          (Transformation|SetRelativeLocation _cube1 (Math|Vector|MakeVector _newtrack_0 (.y _relativelocation) (.z _relativelocation)) false false))))
    (:then_1
      (bind _newtrack_0_2 (Timeline|Timeline_0 Play)
        (:Update
          (Transformation|SetRelativeLocation _cube2 (Math|Vector|MakeVector _newtrack_0_2 (.y _relativelocation_2) (.z _relativelocation_2)) false false))))))

(event OnComponentEndOverlap(Box)
  (params (OverlappedComponent :type Primitive%20Component%20Object%20Reference) (OtherActor :type Actor%20Object%20Reference) (OtherComp :type Primitive%20Component%20Object%20Reference) (OtherBodyIndex :type Integer))
  (bind _cube1 (Variables|Default|GetCube1))
  (bind _cube2 (Variables|Default|GetCube2))
  (bind _relativelocation (Variables|/Script/Engine.SceneComponent|GetRelativeLocation _cube1))
  (bind _relativelocation_2 (Variables|/Script/Engine.SceneComponent|GetRelativeLocation _cube2))
  (Utilities|Casting|CastToPlayer_RebelX OtherActor)
  (Utilities|FlowControl|Sequence
    (:then_0
      (bind _newtrack_0 (Timeline|Timeline Reverse)
        (:Update
          (Transformation|SetRelativeLocation _cube1 (Math|Vector|MakeVector _newtrack_0 (.y _relativelocation) (.z _relativelocation)) false false))))
    (:then_1
      (bind _newtrack_0_2 (Timeline|Timeline_0 Reverse)
        (:Update
          (Transformation|SetRelativeLocation _cube2 (Math|Vector|MakeVector _newtrack_0_2 (.y _relativelocation_2) (.z _relativelocation_2)) false false))))))

(event EventBeginPlay
  (Transformation|SetWorldScale3D (Variables|Default|GetBox) (Variables|Default|GetNew%20Scale)))

(event Collision|EventActorBeginOverlap
  (params (OtherActor :type Actor%20Object%20Reference)))

(event EventTick
  (params (DeltaSeconds :type Float%20%28single-precision%29)))

(fn ConstructionScript)