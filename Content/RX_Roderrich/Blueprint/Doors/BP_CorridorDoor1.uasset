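; Corridor door that slides along its local Z axis when something overlaps its trigger box, unless locked.
; A Timeline drives the mesh on begin overlap and reverses on end overlap, with no active player filter.
; BeginPlay applies trigger scale and door material, darkening the door if locked.
; SetLocked and SetUnlocked toggle the lock and light material, and the OpenDoor event only unlocks.
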(event OnComponentBeginOverlap(Box)
  (params (OverlappedComponent :type Primitive%20Component%20Object%20Reference) (OtherActor :type Actor%20Object%20Reference) (OtherComp :type Primitive%20Component%20Object%20Reference) (OtherBodyIndex :type Integer) (bFromSweep :type Boolean) (SweepResult :type Hit%20Result%20Structure%20%28by%20ref%29))
  (bind _cubegridtooloutput_26f0c6a9 (Variables|Default|GetCubeGridToolOutput_26F0C6A9))
  (bind _relativelocation (Variables|/Script/Engine.SceneComponent|GetRelativeLocation _cubegridtooloutput_26f0c6a9))
  (if (not (Variables|Default|GetLocked))
    (bind _newtrack_0 (Timeline|Timeline Play)
      (:Update
        (Transformation|SetRelativeLocation _cubegridtooloutput_26f0c6a9 (Math|Vector|MakeVector (.x _relativelocation) (.y _relativelocation) _newtrack_0) false false)))))

(event OnComponentEndOverlap(Box)
  (params (OverlappedComponent :type Primitive%20Component%20Object%20Reference) (OtherActor :type Actor%20Object%20Reference) (OtherComp :type Primitive%20Component%20Object%20Reference) (OtherBodyIndex :type Integer))
  (bind _cubegridtooloutput_26f0c6a9 (Variables|Default|GetCubeGridToolOutput_26F0C6A9))
  (bind _relativelocation (Variables|/Script/Engine.SceneComponent|GetRelativeLocation _cubegridtooloutput_26f0c6a9))
  (if (not (Variables|Default|GetLocked))
    (bind _newtrack_0 (Timeline|Timeline Reverse)
      (:Update
        (Transformation|SetRelativeLocation _cubegridtooloutput_26f0c6a9 (Math|Vector|MakeVector (.x _relativelocation) (.y _relativelocation) _newtrack_0) false false)))))

(event EventBeginPlay
  (Transformation|SetWorldScale3D (Variables|Default|GetBox) (Variables|Default|GetNew%20Scale))
  (Rendering|Material|SetMaterial (Variables|Default|GetCubeGridToolOutput_26F0C6A9) 0 (Variables|Default|GetMaterial))
  (if (Variables|Default|GetLocked)
    (Rendering|Material|SetMaterial (Variables|Default|GetLight) 0 "/Game/RX_Roderrich/Materials/Lights/MI_LightCDoor.MI_LightCDoor")
    (Rendering|Material|SetMaterial (Variables|Default|GetCubeGridToolOutput_26F0C6A9) 0 "/Game/RX_Roderrich/Materials/Doors/MI_Metal_Black.MI_Metal_Black")))

(event Collision|EventActorBeginOverlap
  (params (OtherActor :type Actor%20Object%20Reference)))

(event EventTick
  (params (DeltaSeconds :type Float%20%28single-precision%29)))

(event EventOpenDoor
  (params (Rotation :type Float%20%28double-precision%29))
  (CallFunction|SetUnlocked))

(fn ConstructionScript)

(fn SetLocked
  (Variables|Default|SetLocked true)
  (Rendering|Material|SetMaterial (Variables|Default|GetLight) 0 "/Game/RX_Roderrich/Materials/Lights/MI_LightCDoor.MI_LightCDoor"))

(fn SetUnlocked
  (Variables|Default|SetLocked false)
  (Rendering|Material|SetMaterial (Variables|Default|GetLight) 0 "/Game/RX_Roderrich/Materials/Lights/MI_LightODoor.MI_LightODoor"))