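; BP_RoomSigns is a room sign actor that displays editable text, with separate strings for front and back.
; The construction script writes Text and BackText to two TextRender components and applies FontSize as their shared world size when it is non-zero.
; The event graph holds only empty events, so all setup happens at construction.
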(event EventBeginPlay)

(event Collision|EventActorBeginOverlap
  (params (OtherActor :type Actor%20Object%20Reference)))

(event EventTick
  (params (DeltaSeconds :type Float%20%28single-precision%29)))

(fn ConstructionScript
  (Rendering|Components|TextRender|SetText (Variables|Default|GetTextRender1) (Variables|Default|GetText))
  (Rendering|Components|TextRender|SetText (Variables|Default|GetTextRender) (Variables|Default|GetBackText))
  (if (!= (Variables|Default|GetFontSize) 0.0)
    (Rendering|Components|TextRender|SetWorldSize (Variables|Default|GetTextRender) (Variables|Default|GetFontSize))))