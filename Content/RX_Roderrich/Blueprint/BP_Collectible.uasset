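; BP_Collectible is a pickup that the player collects through an interaction prompt showing its item name and the [E] key.
; The construction script either applies the assigned mesh or, in sample mode, hides it and shows sample props with a randomly chosen mesh and an independently randomized material.
; On activation it passes its pickup value to the widget held by GM_RebelX, then destroys itself a tick later.
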(event EventBeginPlay
  (bind _asgm_rebel_x (Utilities|Casting|CastToGM_RebelX (Game|GetGameMode)))
  (Variables|Default|SetAs%20GM%20Rebel%20X _asgm_rebel_x))

(event Collision|EventActorBeginOverlap
  (params (OtherActor :type Actor%20Object%20Reference)))

(event EventTick
  (params (DeltaSeconds :type Float%20%28single-precision%29)))

(event EventActivateSceneObject
  (Default|ValueCalc (Variables|/Game/RebelX_Core/Blueprints/GM_RebelX.GM_RebelX_C|GetWidget (Variables|Default|GetAs%20GM%20Rebel%20X)) (Variables|Default|GetPickupValue))
  (Utilities|FlowControl|DelayUntilNextTick)
  (Actor|DestroyActor))

(fn ConstructionScript
  (bind _object (Variables|Default|GetObject))
  (bind _cube1 (Variables|Default|GetCube1))
  (bind _cube (Variables|Default|GetCube))
  (bind _samplearray (Variables|Default|GetSampleArray))
  (bind _returnvalue (Utilities|Array|LastIndex _samplearray))
  (bind _returnvalue_2 (Math|Random|RandomIntegerinRange 0 _returnvalue))
  (bind _output (Utilities|Array|Get(acopy) _samplearray _returnvalue_2))
  (if (Variables|Default|GetSample)
    (Rendering|SetVisibility _cube1 true false)
    (Components|StaticMesh|SetStaticMesh _cube1 _output)
    (Rendering|Material|SetMaterial _cube1 0 (Rendering|Material|GetMaterial _output 0))
    (Rendering|SetVisibility (Variables|Default|GetCube) false false)
    (else
      (Components|StaticMesh|SetStaticMesh _cube _object)
      (Rendering|Material|SetMaterial _cube 0 (Rendering|Material|GetMaterial _object 0)))))

(fn GetAmmoInfo
  (return false "NewEnumerator0"))

(fn GetCrosshairPrompt
  (return (Utilities|Text|FormatText "Collect {a}" (Variables|Default|GetItem%20Name)) "[E]"))

(fn GetHealthInfo
  (return false 0.0))

(fn GetInteractionType
  (return false "NewEnumerator2"))

(fn GetIsConsumeable
  (return true))

(fn GetSceneInfo
  (return false))