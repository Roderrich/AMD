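; BP_KeyCardDoors is a key card door stub that supplies an "Open Door" crosshair prompt with a "Press [E]" tooltip.
; It implements interface-style queries for interaction, ammo, health, consumable and scene info, which report false alongside placeholder values.
; ActivateSceneObject holds only an always-true branch with no action, so no key check or door movement is implemented here.
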(event EventBeginPlay)

(event Collision|EventActorBeginOverlap
  (params (OtherActor :type Actor%20Object%20Reference)))

(event EventTick
  (params (DeltaSeconds :type Float%20%28single-precision%29)))

(event EventActivateSceneObject
  (if true
    _))

(fn ConstructionScript)

(fn GetAmmoInfo
  (return false "NewEnumerator0"))

(fn GetCrosshairPrompt
  (return "Open Door " "Press [E]"))

(fn GetHealthInfo
  (return false 0.0))

(fn GetInteractionType
  (return false "NewEnumerator2"))

(fn GetIsConsumeable
  (return false))

(fn GetSceneInfo
  (return false))