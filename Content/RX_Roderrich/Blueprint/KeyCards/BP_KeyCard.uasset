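; BP_KeyCard is a keycard pickup that the player collects into their inventory.
; It answers interaction queries with a hover message, an "[E] to Pickup" tooltip, an interaction type and a consumable flag, reporting no ammo, health or scene info.
; On ActivateSceneObject it casts player 0's character to Player_RebelX and adds a true entry to BPCInventory's KeyCards, with no card-specific ID.
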(event EventBeginPlay)

(event Collision|EventActorBeginOverlap
  (params (OtherActor :type Actor%20Object%20Reference)))

(event EventTick
  (params (DeltaSeconds :type Float%20%28single-precision%29)))

(event EventActivateSceneObject
  (bind _asplayer_rebel_x (Utilities|Casting|CastToPlayer_RebelX (Game|GetPlayerCharacter 0)))
  (Utilities|Array|Add (Variables|/Game/RX_Roderrich/BPC_Backpack.BPC_Backpack_C|GetKeyCards (Variables|/Game/RebelX_Core/Blueprints/Player_RebelX.Player_RebelX_C|GetBPC_Inventory _asplayer_rebel_x)) true))

(fn ConstructionScript)

(fn GetAmmoInfo
  (return false "NewEnumerator0"))

(fn GetCrosshairPrompt
  (return (Variables|Default|GetHover%20Message) "[E] to Pickup"))

(fn GetHealthInfo
  (return false 0.0))

(fn GetInteractionType
  (return true "NewEnumerator2"))

(fn GetIsConsumeable
  (return true))

(fn GetSceneInfo
  (return false))