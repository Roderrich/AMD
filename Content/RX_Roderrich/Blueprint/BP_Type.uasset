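; BP_Type is an interactable scene object that opens a typing screen, offered through a "Send Message" crosshair prompt on E.
; BeginPlay creates WBP_Typing once with the actor's RequiredText and binds its Closed event to Close.
; ActivateSceneObject pauses the game, shows the cursor and adds the widget to the viewport; Close reverses all three.
; The other info getters are stubs that return false.
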(event Custom|Close
  (Game|SetGamePaused false)
  (Variables|/Script/Engine.PlayerController|SetbShowMouseCursor (Game|GetPlayerController (Game|GetPlayerState 0)) false)
  (Widget|RemovefromParent (Variables|Default|GetWidget)))

(event EventBeginPlay
  (bind _returnvalue (UserInterface|CreateWidget "/Game/RX_Roderrich/Blueprint/Widgets/WBP_Typing.WBP_Typing_C" 0 (Variables|Default|GetRequired%20Text)))
  (Variables|Default|SetWidget _returnvalue)
  (EventDispatchers|BindEventtoClosed _returnvalue (delegate Custom|Close)))

(event Collision|EventActorBeginOverlap
  (params (OtherActor :type Actor%20Object%20Reference)))

(event EventTick
  (params (DeltaSeconds :type Float%20%28single-precision%29)))

(event EventActivateSceneObject
  (Game|SetGamePaused true)
  (Variables|/Script/Engine.PlayerController|SetbShowMouseCursor (Game|GetPlayerController (Game|GetPlayerState 0)) true)
  (UserInterface|Viewport|AddtoViewport (Variables|Default|GetWidget) 0))

(fn ConstructionScript)

(fn GetAmmoInfo
  (return false "NewEnumerator0"))

(fn GetCrosshairPrompt
  (return "Send Message" "[E]"))

(fn GetHealthInfo
  (return false 0.0))

(fn GetInteractionType
  (return false "NewEnumerator2"))

(fn GetIsConsumeable
  (return false))

(fn GetSceneInfo
  (return false))