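; A crane prop with a crate hanging from a cable and physics constraint, which drops when hit by a light or heavy projectile.
; On play, crane audio starts at a random offset and a timeline slides the arm block between two configurable locations.
; The first projectile hit on the crate destroys the constraint, detaches the cable end and plays a snap sound.
; The construction script positions arm and crate and tints the light through a dynamic material.
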(event OnComponentHit(Crate)
  (params (HitComponent :type Primitive%20Component%20Object%20Reference) (OtherActor :type Actor%20Object%20Reference) (OtherComp :type Primitive%20Component%20Object%20Reference) (NormalImpulse :type Vector :default "0, 0, 0") (Hit :type Hit%20Result%20Structure%20%28by%20ref%29))
  (bind _returnvalue (Utilities|GetClass OtherActor))
  (if (or (== _returnvalue "/Game/RebelX_Core/Blueprints/Projectiles/BP_Projectile_Light.BP_Projectile_Light_C") (== _returnvalue "/Game/RebelX_Core/Blueprints/Projectiles/BP_Projectile_Heavy.BP_Projectile_Heavy_C"))
    (Utilities|FlowControl|DoOnce false
      (:Completed
        (Components|DestroyComponent (Variables|Default|GetPhysicsConstraint))
        (Variables|/Script/CableComponent.CableComponent|SetbAttachEnd (Variables|Default|GetCable) false)
        (Audio|Components|Audio|Play (Variables|Default|GetCableSnap_Cue) 0.0)))))

(event EventBeginPlay
  (Utilities|FlowControl|Sequence
    (:then_0
      (Audio|Components|Audio|Play (Variables|Default|GetCraneAudio) (Math|Random|RandomFloatinRange 0.0 2e+01)))
    (:then_1
      (bind _alpha_lerp (Timeline|MoveArmBlock Play)
        (:Update
          (Transformation|SetRelativeLocation (Variables|Default|GetArmBlock) (Math|Vector|Lerp(Vector) (Variables|Default|GetArmLoc1) (Variables|Default|GetArmLoc2) _alpha_lerp) false false))))))

(event Collision|EventActorBeginOverlap
  (params (OtherActor :type Actor%20Object%20Reference)))

(event EventTick
  (params (DeltaSeconds :type Float%20%28single-precision%29)))

(event Game|Damage|EventAnyDamage
  (params (Damage :type Float%20%28single-precision%29) (DamageType :type Damage%20Type%20Object%20Reference) (InstigatedBy :type Controller%20Object%20Reference) (DamageCauser :type Actor%20Object%20Reference)))

(fn ConstructionScript
  (Transformation|SetRelativeLocation (Variables|Default|GetArmBlock) (Variables|Default|GetArmLoc1) false false)
  (Transformation|SetRelativeLocation (Variables|Default|GetCrate) (Variables|Default|GetCrateStartLoc) false false)
  (bind _returnvalue (Rendering|Material|CreateDynamicMaterialInstance (Variables|Default|GetLight) 0 "/Game/RebelX_Core/Environment/Materials/MI_LightSurface.MI_LightSurface" "SecondaryColor" :!class /Script/Engine.PrimitiveComponent))
  (bind _output_get (Variables|Default|SetLightMaterial _returnvalue))
  (Rendering|Material|SetVectorParameterValue _output_get "SecondaryColor" "(R=1.000000,G=0.491265,B=0.000000,A=1.000000)" :!class /Script/Engine.MaterialInstanceDynamic))