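; BP_OfficeLight is a switchable office light made of a mesh with an emissive-style surface and a rect light.
; The construction script creates a dynamic material instance from MI_LightSurface, then applies the light colour and the initial LightOn state.
; TurnLightOn and TurnLightOff events update LightOn, set the rect light's intensity and swap the material's SecondaryColor between on and off colours.
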(event Custom|TurnLightOn
  (Variables|Default|SetLight%20on true)
  (Rendering|Components|Light|SetIntensity (Variables|Default|GetRectLight) (Variables|Default|GetLight%20Intensity))
  (Rendering|Material|SetVectorParameterValue (Variables|Default|GetLightMaterial) "SecondaryColor" (Variables|Default|GetLightColour) :!class /Script/Engine.MaterialInstanceDynamic))

(event Custom|TurnLightOff
  (Variables|Default|SetLight%20on false)
  (Rendering|Components|Light|SetIntensity (Variables|Default|GetRectLight) 0.0)
  (Rendering|Material|SetVectorParameterValue (Variables|Default|GetLightMaterial) "SecondaryColor" (Variables|Default|GetLightOffColour) :!class /Script/Engine.MaterialInstanceDynamic))

(event EventBeginPlay)

(event Collision|EventActorBeginOverlap
  (params (OtherActor :type Actor%20Object%20Reference)))

(event EventTick
  (params (DeltaSeconds :type Float%20%28single-precision%29)))

(fn ConstructionScript
  (bind _returnvalue (Rendering|Material|CreateDynamicMaterialInstance (Variables|Default|GetLightMesh) 0 "/Game/RebelX_Core/Environment/Materials/MI_LightSurface.MI_LightSurface" "SecondaryColor" :!class /Script/Engine.PrimitiveComponent))
  (bind _output_get (Variables|Default|SetLightMaterial _returnvalue))
  (Rendering|Material|SetVectorParameterValue _output_get "SecondaryColor" (Variables|Default|GetLightColour) :!class /Script/Engine.MaterialInstanceDynamic)
  (Rendering|Components|Light|SetLightColor (Variables|Default|GetRectLight) (Variables|Default|GetLightColour) true)
  (if (Variables|Default|GetLight%20on)
    (Rendering|Components|Light|SetIntensity (Variables|Default|GetRectLight) (Variables|Default|GetLight%20Intensity))
    (else
      (Rendering|Components|Light|SetIntensity (Variables|Default|GetRectLight) 0.0)
      (Rendering|Material|SetVectorParameterValue (Variables|Default|GetLightMaterial) "SecondaryColor" (Variables|Default|GetLightOffColour) :!class /Script/Engine.MaterialInstanceDynamic))))