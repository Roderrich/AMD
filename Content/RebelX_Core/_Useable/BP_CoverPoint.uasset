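; Placeable cover point that describes which low or high, left, center or right cover positions are available at its location.
; The construction script turns its cover flags into a CoverTypes list and shows matching pose and aim preview components, hiding them all when Stand is set.
; GetCoverTypes exposes the list and some flags, while GetCoverTransform returns the matching aim component's world transform with a 90-degree rotation offset.
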(event EventBeginPlay)

(event Collision|EventActorBeginOverlap
  (params (OtherActor :type Actor%20Object%20Reference)))

(event EventTick
  (params (DeltaSeconds :type Float%20%28single-precision%29)))

(fn ConstructionScript
  (bind _left (Variables|CoverType|GetLeft))
  (bind _low_cover (Variables|CoverType|GetLow%20Cover))
  (bind _center (Variables|CoverType|GetCenter))
  (bind _low_cover_2 (Variables|CoverType|GetLow%20Cover))
  (bind _right (Variables|CoverType|GetRight))
  (bind _high_cover (Variables|CoverType|GetHigh%20Cover))
  (bind _right_2 (Variables|CoverType|GetRight))
  (bind _low_cover_3 (Variables|CoverType|GetLow%20Cover))
  (bind _left_2 (Variables|CoverType|GetLeft))
  (bind _high_cover_2 (Variables|CoverType|GetHigh%20Cover))
  (bind _returnvalue (and _low_cover _left))
  (bind _returnvalue_2 (and _low_cover_2 _center))
  (bind _returnvalue_3 (and _high_cover _right))
  (bind _returnvalue_4 (and _low_cover_3 _right_2))
  (bind _returnvalue_5 (and _high_cover_2 _left_2))
  (if (Variables|CoverType|GetStand)
    (Rendering|SetVisibility (Variables|Default|GetHigh%20Pose) false false)
    (else
      (Utilities|FlowControl|Sequence
        (:then_0
          (Utilities|Array|Clear (Variables|Default|GetCover%20Types)))
        (:then_1
          (Utilities|FlowControl|Sequence
            (:then_0
              (Rendering|SetVisibility (Variables|Default|GetLow%20Aim%20Left) _returnvalue false)
              (if _returnvalue
                (Utilities|Array|Add (Variables|Default|GetCover%20Types) "NewEnumerator1")))
            (:then_1
              (Rendering|SetVisibility (Variables|Default|GetLow%20Aim%20Center) _returnvalue_2 false)
              (if _returnvalue_2
                (Utilities|Array|Add (Variables|Default|GetCover%20Types) "NewEnumerator2")))
            (:then_2
              (Rendering|SetVisibility (Variables|Default|GetLow%20Aim%20Right) _returnvalue_4 false)
              (if _returnvalue_4
                (Utilities|Array|Add (Variables|Default|GetCover%20Types) "NewEnumerator3")))
            (:then_4
              (Rendering|SetVisibility (Variables|Default|GetHigh%20Aim%20Left) _returnvalue_5 false)
              (if _returnvalue_5
                (Utilities|Array|Add (Variables|Default|GetCover%20Types) "NewEnumerator4")))
            (:then_5
              (Rendering|SetVisibility (Variables|Default|GetHigh%20Aim%20Right) _returnvalue_3 false)
              (if _returnvalue_3
                (Utilities|Array|Add (Variables|Default|GetCover%20Types) "NewEnumerator5")))
            (:then_6
              (Rendering|SetVisibility (Variables|Default|GetHigh%20Pose) (Variables|CoverType|GetHigh%20Cover) false))))))))

(fn GetCoverTransform
  (params (Cover%20Type :type E_CoverType%20Enum :default "NewEnumerator0"))
  (bind _low_aim_center (Variables|Default|GetLow%20Aim%20Center))
  (bind _low_aim_right (Variables|Default|GetLow%20Aim%20Right))
  (bind _high_aim_left (Variables|Default|GetHigh%20Aim%20Left))
  (bind _high_aim_right (Variables|Default|GetHigh%20Aim%20Right))
  (bind _low_aim_left (Variables|Default|GetLow%20Aim%20Left))
  (bind _defaultsceneroot (Variables|Default|GetDefaultSceneRoot))
  (bind _returnvalue (Utilities|Select :Index Cover%20Type :NewEnumerator0 _defaultsceneroot :NewEnumerator1 _low_aim_left :NewEnumerator2 _low_aim_center :NewEnumerator3 _low_aim_right :NewEnumerator4 _high_aim_left :NewEnumerator5 _high_aim_right))
  (bind _returnvalue_2 (Transformation|GetWorldTransform _returnvalue))
  (bind (_location _rotation _scale) (Math|Transform|BreakTransform _returnvalue_2))
  (return (Math|Transform|MakeTransform _location (Math|Rotator|CombineRotators _rotation "0.000000,90.000000,0.000000") _scale)))

(fn GetCoverTypes
  (return (Variables|CoverType|GetStand) (Variables|Default|GetCover%20Types) (Variables|CoverType|GetRight) (Variables|CoverType|GetLow%20Cover)))