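; BP_LadderVolume is a trigger volume that marks a climbable ladder area for the RebelX player.
; On BeginPlay it caches player 0's character as Player_RebelX.
; Its Box component's begin and end overlap events call OnLadder and OffLadder on that player, ignoring all other actors.
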(event OnComponentBeginOverlap(Box)
  (params (OverlappedComponent :type Primitive%20Component%20Object%20Reference) (OtherActor :type Actor%20Object%20Reference) (OtherComp :type Primitive%20Component%20Object%20Reference) (OtherBodyIndex :type Integer) (bFromSweep :type Boolean) (SweepResult :type Hit%20Result%20Structure%20%28by%20ref%29))
  (bind _as_player_rebel_x (Variables|Default|GetAs%20Player%20Rebel%20X))
  (if (== OtherActor _as_player_rebel_x)
    (Default|OnLadder _as_player_rebel_x)))

(event OnComponentEndOverlap(Box)
  (params (OverlappedComponent :type Primitive%20Component%20Object%20Reference) (OtherActor :type Actor%20Object%20Reference) (OtherComp :type Primitive%20Component%20Object%20Reference) (OtherBodyIndex :type Integer))
  (bind _as_player_rebel_x (Variables|Default|GetAs%20Player%20Rebel%20X))
  (if (== OtherActor _as_player_rebel_x)
    (Default|OffLadder _as_player_rebel_x)))

(event EventBeginPlay
  (bind _asplayer_rebel_x (Utilities|Casting|CastToPlayer_RebelX (Game|GetPlayerCharacter 0)))
  (Variables|Default|SetAs%20Player%20Rebel%20X _asplayer_rebel_x))

(event Collision|EventActorBeginOverlap
  (params (OtherActor :type Actor%20Object%20Reference)))

(event EventTick
  (params (DeltaSeconds :type Float%20%28single-precision%29)))

(fn ConstructionScript)