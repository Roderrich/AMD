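; BP_EncounterControlPoint is an encounter point that tracks the enemies attached to it, up to a target count.
; Activation sets that count and an active flag, and deactivation clears only the flag.
; Attaching adds an enemy uniquely and binds to its destruction, so destroyed or detached enemies leave the list.
; CanAttach reports free slots without checking the flag, and the construction script displays the target as editor text.
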(event Custom|Enemy%20Destroyed
  (params (DestroyedActor :type Actor%20Object%20Reference))
  (Utilities|Array|RemoveItem (Variables|RebelX|EncounterControlPoint|GetEnemies%20At%20Point) DestroyedActor))

(event EventDeactivateControlPoint
  (Variables|RebelX|EncounterControlPoint|SetControl%20Point%20Active false))

(event EventActivateControlPoint
  (params (Enemies%20At%20point :type Integer))
  (Variables|RebelX|EncounterControlPoint|SetTarget%20Enemies%20At%20Point Enemies%20At%20point)
  (Variables|RebelX|EncounterControlPoint|SetControl%20Point%20Active true))

(event EventDetachfromControlPoint
  (params (Enemy :type Actor%20Object%20Reference))
  (Utilities|Array|RemoveItem (Variables|RebelX|EncounterControlPoint|GetEnemies%20At%20Point) (stale Custom|Enemy%20Destroyed DestroyedActor)))

(fn ConstructionScript
  (Rendering|Components|TextRender|SetText (Variables|Default|GetTextRender) (Utilities|Text|FormatText "Target Assigned: {Target}" (Variables|RebelX|EncounterControlPoint|GetTarget%20Enemies%20At%20Point))) ; Update editor info
)

(fn AttachtoControlPoint
  (params (Enemy :type Actor%20Object%20Reference))
  (bind _enemies_at_point (Variables|RebelX|EncounterControlPoint|GetEnemies%20At%20Point))
  (if (not (Utilities|Array|ContainsItem _enemies_at_point Enemy))
    (Utilities|Array|Add _enemies_at_point Enemy)
    (Game|BindEventtoOnDestroyed Enemy (EventDispatchers|CreateEvent :!event Custom|Enemy%20Destroyed))))

(fn CanAttach
  (return (> (- (Variables|RebelX|EncounterControlPoint|GetTarget%20Enemies%20At%20Point) 1) (Utilities|Array|LastIndex (Variables|RebelX|EncounterControlPoint|GetEnemies%20At%20Point)))))

(fn GetAttachedEnemies
  (return (Variables|RebelX|EncounterControlPoint|GetEnemies%20At%20Point)))