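; Interactable ammo pickup that offers a refill of all ammo at the "[E] PICKUP" prompt.
; It answers interaction queries with its type and a map granting the same AmmoAmount to eight ammo types, while reporting no health or scene info.
; It reports itself as non-consumable and leaves the consume event empty.
; The construction script does nothing, with leftover dynamic-material Decal setup left disconnected.
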(event EventAttemptConsumeInteractable)

(fn ConstructionScript)

(fn GetInteractionType
  (return true "NewEnumerator1"))

(fn GetAmmoInfo
  (bind _ammo_amount (Variables|Default|GetAmmo%20Amount))
  (bind _returnvalue (Class|KismetSystemLibrary|MakeLiteralInteger _ammo_amount))
  (return true (Utilities|Map|MakeMap "NewEnumerator5" _returnvalue "NewEnumerator4" _returnvalue "NewEnumerator2" _returnvalue "NewEnumerator1" _returnvalue "NewEnumerator6" _returnvalue "NewEnumerator3" _returnvalue "NewEnumerator7" _returnvalue "NewEnumerator0" _returnvalue)))

(fn GetCrosshairPrompt
  (return "REFILL ALL AMMO" "[E] PICKUP"))

(fn GetIsConsumeable
  (return false))

(fn GetSceneInfo
  (return false))

(fn GetHealthInfo
  (return false 0.0))