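; Rocket projectile Blueprint that turns the parent projectile's hit response into an area explosion.
; It overrides the damage step to apply radial falloff damage between inner and outer sphere components, using damage and type from its projectile data.
; It overrides the physics step to overlap nearby components within the outer radius and push each with a linear-falloff radial impulse applied as a velocity change.
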(event EventBeginPlay
  (|CallParentFunction) ; This node is disabled and will not be called.\nDrag off pins to build functionality.
)

(event EventAddPhysicsImpule
  (bind _returnvalue (Transformation|GetActorLocation))
  (bind _explosionradius_outer (Variables|Default|GetExplosionRadius_Outer))
  (bind _sphereradius (Variables|/Script/Engine.SphereComponent|GetSphereRadius _explosionradius_outer))
  ;[1 1 1] Override physics to shpere
  (bind _outcomponents (Collision|SphereOverlapComponents _returnvalue _sphereradius (Utilities|Array|MakeArray "ObjectTypeQuery2" "ObjectTypeQuery3" "ObjectTypeQuery4" "ObjectTypeQuery5" "ObjectTypeQuery6") "/Script/Engine.PrimitiveComponent"))
  (for _array_element _outcomponents
    (Physics|AddRadialImpulse _array_element _returnvalue _sphereradius (Variables|Default|GetPhysicsImpulseStrength) "RIF_Linear" true)))

(event EventApplyDamagetoHit
  (bind _projectiledata (Variables|Default|GetProjectileData))
  (bind (_projectileclass _damagetype _damage) (Utilities|Struct|BreakS_Projectile _projectiledata))
  ;[1 1 1] Override Damage to sphere
  (Class|GameplayStatics|ApplyRadialDamagewithFalloff _damage 0.0 (Transformation|GetActorLocation) (Variables|/Script/Engine.SphereComponent|GetSphereRadius (Variables|Default|GetExplosionRadius_Inner)) (Variables|/Script/Engine.SphereComponent|GetSphereRadius (Variables|Default|GetExplosionRadius_Outer)) 1.0 _damagetype 0 self (Pawn|GetController (Variables|Default|GetInstigator)) "ECC_Visibility"))

(fn ConstructionScript
  (|CallParentFunction))