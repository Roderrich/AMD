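; Combat manager component that tracks enemies, encounters and combat state, with optional music, chimes and debug printout.
; Adding an enemy targets it on the player, sets its stance and alerts it; the first starts combat and pulls in active enemies from attached encounters.
; It arbitrates a shared attack-token pool and cover-point reservations through request and return calls.
; Removing enemies does not end combat, and nothing here calls EndCombat.
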(event Custom|End%20Combat%20Music
  (bind _combatmusic (Variables|Default|GetCombatMusic))
  ;[1 1 1] Music
  (Utilities|FlowControl|Delay 1.0)
  (Utilities|FlowControl|Sequence
    (:then_0
      (if (Variables|RebelX|CombatManager|Audio|GetCombat%20Chimes)
        (Audio|PlaySound2D "/Game/RebelX_Core/Audio/FX/SC_FX_CombatEnded.SC_FX_CombatEnded" 2.0 1.0 0.0 0 0)))
    (:then_1
      (Utilities|IsValid _combatmusic
        (:Is%20Valid
          (Audio|Components|Audio|Stop _combatmusic)
          (Components|DestroyComponent _combatmusic))))))

(event Custom|Start%20Combat%20Music
  (Utilities|FlowControl|Sequence
    (:then_0
      (if (Variables|RebelX|CombatManager|Audio|GetCombat%20Chimes)
        ;[1 1 0] Need music system
        (Audio|PlaySound2D "/Game/RebelX_Core/Audio/FX/SC_FX_CombatStarted.SC_FX_CombatStarted" 2.0 1.0 0.0 0 0)
        (Audio|PlaySound2D "/Game/RebelX_Core/Audio/FX/W_FX_CombatStarted.W_FX_CombatStarted" 0.5 1.0 0.0 0 0)))
    (:then_1
      ;[1 1 0] Combat Music
      (if (Variables|RebelX|CombatManager|Audio|GetCombat%20Music)
        (Utilities|IsValid (Variables|Default|GetCombatMusic)
          (:Is%20Not%20Valid
            (bind _returnvalue (Audio|SpawnSoundAttached "/Game/RebelX_Core/Audio/FX/W_CombatMusic.W_CombatMusic" (Variables|/Script/Engine.Actor|GetRootComponent (Game|Player|GetPlayerPawn 0)) "None" "0, 0, 0" "0, 0, 0" "KeepRelativeOffset" false 1.0 1.0 0.0 0 0))
            (bind _output_get (Variables|Default|SetCombatMusic _returnvalue))
            (Class|AudioComponent|SetUISound _output_get true)))))))

(event EventReturnCoverPoint
  (params (Cover%20Point :type Actor%20Object%20Reference))
  ;[1 1 1] Return Cover Point
  (Utilities|Map|Remove (Variables|RebelX|CombatManager|Encounters|GetOccupied%20Cover%20Points) Cover%20Point))

(event EventAddtoCombat
  (params (Actor :type Actor%20Object%20Reference))
  ;[1 1 1] Add to Combat
  (Utilities|FlowControl|DelayUntilNextTick)
  (Utilities|FlowControl|Sequence
    (:then_0
      (if (not (Utilities|Map|Contains (Variables|RebelX|CombatManager|Encounters|GetEnemy%20Characters) Actor))
        (|GraphAddToCombat Actor)
        (elif (Variables|RebelX|GetDebug)
          (CallFunction|DebugLog "Enemy Already added to combat." "NewEnumerator1" "None" false))))
    (:then_1
      (if (not (Variables|RebelX|CombatManager|GetCombat%20Active))
        (CallFunction|StartCombat)
        (CallFunction|AlertEnemeisfromAttachedEncounter Actor)))))

(event EventRemoveEncounterManager
  (params (Encounter%20Manager :type Actor%20Object%20Reference))
  ;[1 1 1] Remove Encounter
  (Utilities|Set|Remove (Variables|RebelX|CombatManager|Encounters|GetCurrent%20Encounters) Encounter%20Manager))

(event EventRemovefromCombat
  (params (Actor :type Actor%20Object%20Reference))
  ;[1 1 1] Remove From Combat
  (Utilities|Map|Remove (Variables|RebelX|CombatManager|Encounters|GetEnemy%20Characters) Actor)
  (CallFunction|DebugLog (Utilities|String|Append "Removing enemy from combat: " (Utilities|GetDisplayName Actor)) "NewEnumerator0" "None" (Variables|RebelX|GetDebug)))

(event EventAttachEncounterManager
  (params (Encounter%20Manager :type Actor%20Object%20Reference))
  ;[1 1 1] Attach Encounter
  (Utilities|Set|Add (Variables|RebelX|CombatManager|Encounters|GetCurrent%20Encounters) Encounter%20Manager)
  (if (Variables|RebelX|CombatManager|GetCombat%20Active)
    (CallFunction|AlertEnemeisfromAttachedEncounter)))

(event EventBeginPlay
  (if (Variables|RebelX|GetDebugInfo)
    (Components|Tick|SetComponentTickEnabled true)))

(event EventTick
  (params (DeltaSeconds :type Float%20%28single-precision%29))
  (CallFunction|PrintDebugInfo))

(event EventResetAttackTokens
  (params (Attack%20Tokens :type Integer))
  ;[1 1 1] Reset Attack Tokens
  (Variables|RebelX|CombatManager|SetAvalible%20Attack%20Tokens Attack%20Tokens))

(fn SendtoAttack
  (params (Charachter :type Character%20Object%20Reference))
  (AI|Components|Blackboard|SetValueasEnum (AI|GetBlackboard (AI|GetAIController Charachter)) (Utilities|Name|MakeLiteralName "Stance") (Utilities|Enum|LiteralenumE_EnemyStances "NewEnumerator1")))

(fn UpdateCombatMusicConfig
  (params (bPlayCombatMusic :type Boolean) (bPlayCombatChimes :type Boolean))
  (Variables|RebelX|CombatManager|Audio|SetCombat%20Music bPlayCombatMusic)
  (Variables|RebelX|CombatManager|Audio|SetCombat%20Chimes bPlayCombatChimes))

(fn AlertEnemeisfromAttachedEncounter
  (params (Alerter :type Actor%20Object%20Reference))
  (bind _result (Utilities|Set|ToArray (Variables|RebelX|CombatManager|Encounters|GetCurrent%20Encounters)))
  (for _array_element _result
    (bind _enemies (Class|BPIEncounterManager|GetActiveEnemies(Message) _array_element))
    (Utilities|Array|RemoveItem _enemies Alerter)
    (for _array_element_2 _enemies
      (CallFunction|AddtoCombat _array_element_2))))

(fn StartCombat
  (CallFunction|DebugLog "Starting Combat..." "NewEnumerator0" "Combat" (Variables|RebelX|GetDebug))
  (Variables|RebelX|CombatManager|SetCombat%20Active true)
  (Default|CallCombatStarted)
  (CallFunction|StartCombatMusic))

(fn EndCombat
  (CallFunction|DebugLog "Ending Combat..." "NewEnumerator0" "Combat" (Variables|RebelX|GetDebug))
  (Variables|RebelX|CombatManager|SetCombat%20Active false)
  (Default|CallCombatEnded)
  (CallFunction|EndCombatMusic))

(fn PrintDebugInfo
  (Utilities|FlowControl|Sequence
    (:then_0
      (Development|PrintString "COMBAT MANAGER DEBUG" true true "(R=1.000000,G=0.000000,B=0.027671,A=1.000000)" 2.0 "Debug Header"))
    (:then_1
      (Development|PrintString (Utilities|String|Append "AVALIBLE ATTACK TOKENS = " (Utilities|String|ToString(Integer) (Variables|RebelX|CombatManager|GetAvalible%20Attack%20Tokens))) true true "(R=1.000000,G=1.000000,B=1.000000,A=1.000000)" 2.0 "Tokens"))
    (:then_2
      (Development|PrintString "ATTACTHED ENEMIES 
--------------------- " true true "(R=1.000000,G=1.000000,B=1.000000,A=1.000000)" 2.0 "Enemeis Header")
      (bind _keys (Utilities|Map|Keys (Variables|RebelX|CombatManager|Encounters|GetEnemy%20Characters)))
      (for _array_element _keys
        (LocalVariables|SetEnemies (Utilities|String|Append (Utilities|GetDisplayName _array_element) " 
" (LocalVariables|GetEnemies))))
      (Development|PrintString (LocalVariables|GetEnemies) true true "(R=1.000000,G=1.000000,B=1.000000,A=1.000000)" 2.0 "Enemies"))
    (:then_3
      (Development|PrintString "ATTATCHED ENCOUNTERS 
-------------------------- " true true "(R=1.000000,G=1.000000,B=1.000000,A=1.000000)" 2.0 "Encounter Header")
      (bind _result (Utilities|Set|ToArray (Variables|RebelX|CombatManager|Encounters|GetCurrent%20Encounters)))
      (for _array_element_2 _result
        (LocalVariables|SetEncounters (Utilities|String|Append (Utilities|GetDisplayName _array_element_2) " 
" (LocalVariables|GetEncounters))))
      (Development|PrintString (LocalVariables|GetEncounters) true true "(R=1.000000,G=1.000000,B=1.000000,A=1.000000)" 2.0 "Encounters"))
    (:then_5
      (Development|PrintString "ATTATCHED COVER POINTS 
------------------------------" true true "(R=1.000000,G=1.000000,B=1.000000,A=1.000000)" 2.0 "Control Point Header")
      (bind _keys_2 (Utilities|Map|Keys (Variables|RebelX|CombatManager|Encounters|GetOccupied%20Cover%20Points)))
      (for _array_element_3 _keys_2
        (LocalVariables|SetCover%20Points (Utilities|String|Append (Utilities|GetDisplayName _array_element_3) " 
" (LocalVariables|GetCover%20Points))))
      (Development|PrintString (LocalVariables|GetCover%20Points) true true "(R=1.000000,G=1.000000,B=1.000000,A=1.000000)" 2.0 "Control Points"))))

(fn InCombat
  (return (Variables|RebelX|CombatManager|GetCombat%20Active)))

(fn RequestAttackTokens
  (params (Requested%20Attack%20Tokens :type Integer))
  (if (<= Requested%20Attack%20Tokens (Variables|RebelX|CombatManager|GetAvalible%20Attack%20Tokens))
    (bind _output_get (Variables|RebelX|CombatManager|SetAvalible%20Attack%20Tokens (- (Variables|RebelX|CombatManager|GetAvalible%20Attack%20Tokens) Requested%20Attack%20Tokens)))
    (CallFunction|DebugLog (Utilities|String|Append "Attack Tokens: " (Utilities|String|ToString(Integer) _output_get)) "NewEnumerator0" "Attack Tokens" (Variables|RebelX|GetDebug))
    (return true Requested%20Attack%20Tokens)
    (else
      (return false 0))))

(fn RequestCoverPoint
  (params (CoverPoint :type Actor%20Object%20Reference))
  (if (not (.ReturnValue (Utilities|Map|Find (Variables|RebelX|CombatManager|Encounters|GetOccupied%20Cover%20Points) CoverPoint)))
    (Utilities|Map|Add (Variables|RebelX|CombatManager|Encounters|GetOccupied%20Cover%20Points) CoverPoint true)
    (return true CoverPoint)
    (else
      (return false 0))))

(fn ReturnAttackTokens
  (params (Attack%20Tokens :type Integer))
  (bind _output_get (Variables|RebelX|CombatManager|SetAvalible%20Attack%20Tokens (+ Attack%20Tokens (Variables|RebelX|CombatManager|GetAvalible%20Attack%20Tokens))))
  (CallFunction|DebugLog (Utilities|String|Append "Attack Tokens: " (Utilities|String|ToString(Integer) _output_get)) "NewEnumerator0" "Attack Tokens" (Variables|RebelX|GetDebug))
  (return true))