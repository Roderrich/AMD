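; LRAF9 launcher weapon Blueprint, a child of the LPAMG weapon base that tailors attachments and pickup prompt to this launcher.
; Construction creates a render target for the scope camera and feeds it into a dynamic material on the scope mesh, giving a live picture-in-picture scope.
; Overrides remap attachment parents, point magazine and reserve to rocket sockets, tie ironsight visibility to the selected scope, and leave several attachment icon getters empty.
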(fn ConstructionScript
  (|CallParentFunction)
  (bind _returnvalue (Rendering|CreateRenderTarget2D 512 512 "RTF_RGBA16f"))
  (Variables|/Script/Engine.SceneCaptureComponent2D|SetTextureTarget (Variables|Default|GetScope%20Render%20Camera) _returnvalue)
  (bind _returnvalue_2 (Rendering|Material|CreateDynamicMaterialInstance (Variables|Default|GetMesh%20Scope) 5 "/Game/RebelX_Core/Weapons/_Common/Materials/MI_LPAMG_ATT_Scope_LRAF9_Render.MI_LPAMG_ATT_Scope_LRAF9_Render" "None" :!class /Script/Engine.PrimitiveComponent))
  (Rendering|Material|SetTextureParameterValue _returnvalue_2 "Render Texture" _returnvalue))

(fn LPAMG-GetTextureIconMuzzle
  (return 0))

(fn LPAMG-GetTextureIconForestock
  (return 0))

(fn LPAMG-GetTextureIconIronsightsFront
  (return 0))

(fn LPAMG-GetTextureIconIronsightsBack
  (return 0))

(fn GetSocketGripParent
  (return (Variables|Default|GetWeapon) (.Socket%20Name (|CallParentFunction))))

(fn GetSocketMuzzleParent
  (return (Variables|Default|GetWeapon) (.Socket%20Name (|CallParentFunction))))

(fn GetSocketLaserParent
  (return 0 (.Socket%20Name (|CallParentFunction))))

(fn GetIronsightVisibility
  (return (Utilities|Select :Index (Utilities|Array|FindItem (Variables|Default|GetArray%20Static%20Mesh%20Scopes) (Variables|/Script/Engine.StaticMeshComponent|GetStaticMesh (Variables|Default|GetMesh%20Scope))) :Option%200 true :Option%201 false :Option%202 false)))

(fn LPAMG-GetTextureIconBipod
  (return 0))

(fn GetSocketScopeParent
  (return (Variables|Default|GetRail) (.Socket%20Name (|CallParentFunction))))

(fn GetSocketMagazineParent
  (return (.Parent (|CallParentFunction)) "SOCKET_Rocket"))

(fn GetSocketMagazineReserveParent
  (return (.Parent (|CallParentFunction)) "SOCKET_Rocket_Reserve"))

(fn LPAMG-ShouldApplyWorldspaceScopeOffset
  (return 0.0))

(fn GetCrosshairPrompt
  (return "LRAF9 - LAUNCHER" "[E] PICKUP"))