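; HUD Blueprint for RebelX that builds the player's on-screen UI and exposes events for other gameplay code to drive it.
; On BeginPlay it casts the controlled pawn to Player_RebelX, then creates the HUDCore widget with that player's health component and adds it to the player screen.
; Its events forward to HUDCore and its child widgets for visibility, hit markers, crosshair prompts, queued notifications, mission details and objective updates.
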(event Custom|SetCrosshair_1
  ;[1 1 1] Create crosshair
)

(event EventBeginPlay
  ;[1 1 1] Get player reference
  (bind _asplayer_rebel_x (Utilities|Casting|CastToPlayer_RebelX (Pawn|GetControlledPawn (Game|Player|GetOwningPlayerController)))
    (:then
      (Variables|Default|SetPlayerReference _asplayer_rebel_x)
      (Utilities|FlowControl|Sequence
        (:then_0
          (Utilities|FlowControl|Sequence
            (:then_0
              ;[1 1 1] Create HUD
              (bind _returnvalue (UserInterface|CreateWidget "/Game/RebelX_Core/UserInterface/HUDCore.HUDCore_C" (Game|Player|GetOwningPlayerController) (Variables|/Game/RebelX_Core/Blueprints/Player_RebelX.Player_RebelX_C|GetBP_Health%20Component (Variables|Default|GetPlayerReference))))
              (bind _output_get (Variables|Default|SetHUDCore _returnvalue))
              (UserInterface|Viewport|AddtoPlayerScreen _output_get))))))
    (:CastFailed
      (CallFunction|DebugLog "Cast to player charachter failed" "NewEnumerator2" "None" false))))

(event EventShowCrosshairPrompt
  (params (Prompt :type Text) (Type :type E_CrosshairPromptTpye%20Enum :default "NewEnumerator0"))
  ;[1 1 1] Croshair Prompt
  (Default|ShowPromptforDuration (Variables|/Game/RebelX_Core/UserInterface/HUDCore.HUDCore_C|GetWC_CursorPrompt (Variables|Default|GetHUDCore)) Prompt Type 1.0))

(event EventShowAllUI
  (Widget|SetVisibility (Variables|Default|GetHUDCore) "Visible"))

(event EventToggleMissionDetails
  ;[1 1 1] Toggle Mission Details
  (Default|ToggleDisplay (Variables|/Game/RebelX_Core/UserInterface/HUDCore.HUDCore_C|GetWC_MissionDetails (Variables|Default|GetHUDCore))))

(event EventAddNotificaiton
  (params (NotificationText :type Text))
  ;[1 1 1] Add Hud Notification to Que
  (Default|AddNotificationtoQue (Variables|/Game/RebelX_Core/UserInterface/HUDCore.HUDCore_C|GetW_HUDNotification (Variables|Default|GetHUDCore)) NotificationText))

(event EventShowHitMarker
  ;[1 1 1] Show Hit Marker
  (Default|ShowHitMarker (Variables|/Game/RebelX_Core/UserInterface/HUDCore.HUDCore_C|GetWBP_LPAMG_Crosshair (Variables|Default|GetHUDCore))))

(event EventUpdateObjective
  (params (Objective :type Text) (Details :type Text))
  ;[1 1 1] Update Objective
  (Default|EventUpdateObjective (Variables|Default|GetHUDCore) Objective Details))

(event EventHideAllUI
  (Widget|SetVisibility (Variables|Default|GetHUDCore) "Hidden"))

(fn ConstructionScript)