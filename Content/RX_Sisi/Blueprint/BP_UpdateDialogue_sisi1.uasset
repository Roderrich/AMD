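; BP_UpdateDialogue_sisi1 is a one-shot trigger volume that shows dialogue when the player enters its box.
; The first overlap by Player_RebelX passes the configured row name, data table and time to GetDialogue on the player's widget.
; After a fixed delay, independent of that time value, it fires the Dialoguefinished dispatcher and destroys itself.
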(event OnComponentBeginOverlap(Box)
  (params (OverlappedComponent :type Primitive%20Component%20Object%20Reference) (OtherActor :type Actor%20Object%20Reference) (OtherComp :type Primitive%20Component%20Object%20Reference) (OtherBodyIndex :type Integer) (bFromSweep :type Boolean) (SweepResult :type Hit%20Result%20Structure%20%28by%20ref%29))
  ;[0.15 0.15 0.15 0.5] 是否拾取了0号卡
  (bind _asplayer_rebel_x (Utilities|Casting|CastToPlayer_RebelX OtherActor))
  (Utilities|FlowControl|DoOnce false
    (:Completed
      (Default|GetDialogue (Variables|/Game/RebelX_Core/Blueprints/Player_RebelX.Player_RebelX_C|GetWidget _asplayer_rebel_x) (Variables|Default|GetRow%20Name) (Variables|Default|GetData%20Table) (Variables|Default|GetTime))
      (CallFunction|Dialoguefinished))))

(event Custom|dialoguefinished
  (Utilities|FlowControl|Delay 7.0)
  (Default|CallDialoguefinished)
  (Actor|DestroyActor))

(event EventBeginPlay)

(event Collision|EventActorBeginOverlap
  (params (OtherActor :type Actor%20Object%20Reference)))

(event EventTick
  (params (DeltaSeconds :type Float%20%28single-precision%29)))

(fn ConstructionScript)