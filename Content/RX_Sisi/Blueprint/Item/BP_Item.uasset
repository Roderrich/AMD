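; BP_Item is a pickup actor that the player collects with E while inside its sphere, adding the item's value to a running total.
; On BeginPlay it loads its data from the fixed "Sample" row of DT_Item.
; Sphere overlap toggles the prompt widget, input and a Gate that lets E through.
; Pickup briefly shows "+value" in UI_valueitem, adds it to the INS_Data game instance, then destroys the actor.
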(event OnComponentBeginOverlap(Sphere)
  (params (OverlappedComponent :type Primitive%20Component%20Object%20Reference) (OtherActor :type Actor%20Object%20Reference) (OtherComp :type Primitive%20Component%20Object%20Reference) (OtherBodyIndex :type Integer) (bFromSweep :type Boolean) (SweepResult :type Hit%20Result%20Structure%20%28by%20ref%29))
  (bind _str_item (Variables|Default|GetSTR_item))
  (bind _value (Utilities|Struct|BreakStruct_item _str_item))
  (if (== (Game|Player|GetPlayerPawn 0) OtherActor)
    (Utilities|FlowControl|Sequence
      (:then_0
        (Utilities|FlowControl|Delay 0.2)
        (Development|SetHiddeninGame (Variables|Default|GetWidget) false false))
      (:then_1
        (Input|EnableInput (Game|GetPlayerController 0))
        (Utilities|FlowControl|Gate true) ; enters at Open
      ))))

(event OnComponentEndOverlap(Sphere)
  (params (OverlappedComponent :type Primitive%20Component%20Object%20Reference) (OtherActor :type Actor%20Object%20Reference) (OtherComp :type Primitive%20Component%20Object%20Reference) (OtherBodyIndex :type Integer))
  (bind _str_item (Variables|Default|GetSTR_item))
  (bind _value (Utilities|Struct|BreakStruct_item _str_item))
  (if (== (Game|Player|GetPlayerPawn 0) OtherActor)
    (Utilities|FlowControl|Sequence
      (:then_0
        (Input|DisableInput (Game|GetPlayerController 0))
        (Utilities|FlowControl|Gate true) ; enters at Close
      )
      (:then_1
        (Development|SetHiddeninGame (Variables|Default|GetWidget) true false)))))

(event EventBeginPlay
  (bind _returnvalue (Utilities|GetDataTableRow "/Game/RX_Sisi/Blueprint/DT_Item.DT_Item" "Sample")
    (:then
      (Variables|Default|SetSTR_item _returnvalue))))

(event Collision|EventActorBeginOverlap
  (params (OtherActor :type Actor%20Object%20Reference)))

(event EventTick
  (params (DeltaSeconds :type Float%20%28single-precision%29)))

(event Input|KeyboardEvents|E
  (params (Key :type Key%20Structure :default "None"))
  (bind _str_item (Variables|Default|GetSTR_item))
  (bind _value (Utilities|Struct|BreakStruct_item _str_item))
  (:Pressed
    (Utilities|FlowControl|Gate true
      (:Exit
        (bind _foundwidgets (Widget|GetAllWidgetsOfClass "/Game/RX_Sisi/UI/UI_valueitem.UI_valueitem_C" true))
        (bind _output_get (Variables|Default|Setui_valueitem (Utilities|Array|Get(acopy) _foundwidgets)))
        (Variables|/Game/RX_Sisi/UI/UI_valueitem.UI_valueitem_C|Setaddvaluenum (Utilities|Array|Get(acopy) _foundwidgets) (Utilities|Text|ToText(String) (Utilities|String|Append "+ " (Utilities|String|ToString(Integer) _value))))
        (Variables|/Script/UMG.Widget|SetVisibility (Variables|/Game/RX_Sisi/UI/UI_valueitem.UI_valueitem_C|Getaddvalue _output_get) "Visible")
        (Utilities|FlowControl|Sequence
          (:then_0
            (Utilities|FlowControl|Delay 1.5)
            (Variables|/Script/UMG.Widget|SetVisibility (Variables|/Game/RX_Sisi/UI/UI_valueitem.UI_valueitem_C|Getaddvalue _output_get) "Hidden")
            (Actor|DestroyActor))
          (:then_1
            (bind _asins_data (Utilities|Casting|CastToINS_Data (Game|GetGameInstance)))
            (Variables|/Game/RX_Sisi/Blueprint/INS_Data.INS_Data_C|SetValue _asins_data (+ (Variables|/Game/RX_Sisi/Blueprint/INS_Data.INS_Data_C|GetValue _asins_data) _value))))))))

(fn ConstructionScript)