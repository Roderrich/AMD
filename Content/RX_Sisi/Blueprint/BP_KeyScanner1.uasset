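; Key scanner actor that unlocks when a player carrying the required key card enters its box trigger.
; The overlap checks the player's backpack key cards against the needed ID and clears the Locked flag.
; Activating it while unlocked opens a fingerprint UI widget, passes it an actor reference and switches to UI-only input with a cursor.
; Its crosshair prompt reflects the lock state, while the other info getters return stub values.
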(event OnComponentBeginOverlap(Box)
  (params (OverlappedComponent :type Primitive%20Component%20Object%20Reference) (OtherActor :type Actor%20Object%20Reference) (OtherComp :type Primitive%20Component%20Object%20Reference) (OtherBodyIndex :type Integer) (bFromSweep :type Boolean) (SweepResult :type Hit%20Result%20Structure%20%28by%20ref%29))
  (bind _asplayer_rebel_x (Utilities|Casting|CastToPlayer_RebelX OtherActor))
  (if (Utilities|Array|Get(acopy) (Variables|/Game/RX_Roderrich/BPC_Backpack.BPC_Backpack_C|GetKeyCards (Variables|/Game/RebelX_Core/Blueprints/Player_RebelX.Player_RebelX_C|GetBPC_Backpack _asplayer_rebel_x)) (Variables|Default|GetID%20Needed))
    (CallFunction|ClearanceAquirred)))

(event Custom|ClearanceAquirred
  (Variables|Default|SetLocked false))

(event EventBeginPlay)

(event Collision|EventActorBeginOverlap
  (params (OtherActor :type Actor%20Object%20Reference)))

(event EventActivateSceneObject
  (bind _returnvalue (Game|GetPlayerController 0))
  (if (not (Variables|Default|GetLocked))
    (bind _returnvalue_2 (UserInterface|CreateWidget "/Game/RX_Sisi/UI/UI_Fingureprint.UI_Fingureprint_C" _returnvalue))
    (Variables|/Game/RX_Sisi/UI/UI_Fingureprint.UI_Fingureprint_C|SetACTOR _returnvalue_2 (Variables|Default|GetACTOR))
    (UserInterface|Viewport|AddtoViewport _returnvalue_2 0)
    (Input|SetInputModeUIOnly _returnvalue 0 "DoNotLock" false)
    (Variables|/Script/Engine.PlayerController|SetbShowMouseCursor _returnvalue true)
    (Widget|SetFocus _returnvalue_2)))

(fn ConstructionScript)

(fn GetAmmoInfo
  (return false "NewEnumerator0"))

(fn GetCrosshairPrompt
  (if (Variables|Default|GetLocked)
    (return (Variables|Default|GetLocked%20Message) "")
    (else
      (return (Variables|Default|GetUnlocked%20Message) "[E]"))))

(fn GetHealthInfo
  (return false 0.0))

(fn GetInteractionType
  (return false "NewEnumerator2"))

(fn GetIsConsumeable
  (return false))

(fn GetSceneInfo
  (return false))