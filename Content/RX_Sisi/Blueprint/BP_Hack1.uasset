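; BP_Hack1 is an interactable hack point that starts a timed hack when the player activates it.
; Activation, gated by a DoOnce, spawns a control-room dialogue actor from the "hacking" DT_SISI row, starts the GM_RebelX widget's hack, fires an encounter message and broadcasts HackStarted.
; The widget's completion callback clears the crosshair prompt and broadcasts HackFinished.
; Overlap volume R flags the widget whenever an AI soldier enters or leaves range.
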(event OnComponentBeginOverlap(r)
  (params (OverlappedComponent :type Primitive%20Component%20Object%20Reference) (OtherActor :type Actor%20Object%20Reference) (OtherComp :type Primitive%20Component%20Object%20Reference) (OtherBodyIndex :type Integer) (bFromSweep :type Boolean) (SweepResult :type Hit%20Result%20Structure%20%28by%20ref%29))
  (Utilities|Casting|CastToAI_Soldier_Child OtherActor)
  (Variables|/Game/RX_Roderrich/Blueprint/Widgets/WBP_Additional.WBP_Additional_C|SetEnemyinRange (Variables|/Game/RebelX_Core/Blueprints/GM_RebelX.GM_RebelX_C|GetWidget (Variables|Default|GetAs%20GM%20Rebel%20X)) true))

(event OnComponentEndOverlap(r)
  (params (OverlappedComponent :type Primitive%20Component%20Object%20Reference) (OtherActor :type Actor%20Object%20Reference) (OtherComp :type Primitive%20Component%20Object%20Reference) (OtherBodyIndex :type Integer))
  (Utilities|Casting|CastToAI_Soldier_Child OtherActor)
  (Variables|/Game/RX_Roderrich/Blueprint/Widgets/WBP_Additional.WBP_Additional_C|SetEnemyinRange (Variables|/Game/RebelX_Core/Blueprints/GM_RebelX.GM_RebelX_C|GetWidget (Variables|Default|GetAs%20GM%20Rebel%20X)) false))

(event Custom|CustomEvent
  (Utilities|FlowControl|DoOnce false) ; enters at Reset
)

(event Custom|HackFinished_Event
  (Variables|Default|SetPrompt "")
  (Variables|Default|SetTooltip "")
  (Default|CallHackFinished))

(event EventBeginPlay)

(event Collision|EventActorBeginOverlap
  (params (OtherActor :type Actor%20Object%20Reference)))

(event EventTick
  (params (DeltaSeconds :type Float%20%28single-precision%29)))

(event EventActivateSceneObject
  (Utilities|FlowControl|DoOnce false
    (:Completed
      (Game|SpawnActorfromClass "/Game/RX_Sisi/Blueprint/Dialogue/BP_Dia_controlroom.BP_Dia_controlroom_C" (Math|Transform|MakeTransform (Transformation|GetActorLocation (Game|Player|GetPlayerPawn 0)) "0, 0, 0" "3.000000,3.000000,3.000000") "Undefined" "MultiplyWithRoot" 0 "hacking" "/Game/RX_Sisi/DATATABLE/DT_SISI.DT_SISI" 0.02 0)
      (bind _asgm_rebel_x (Utilities|Casting|CastToGM_RebelX (Game|GetGameMode)))
      (bind _output_get (Variables|Default|SetAs%20GM%20Rebel%20X _asgm_rebel_x))
      (Default|HackEvent (Variables|/Game/RebelX_Core/Blueprints/GM_RebelX.GM_RebelX_C|GetWidget _output_get) (Variables|Default|GetTime))
      (Class|BPIEncounterManager|ActivateEncounter(Message) (Variables|Default|GetActor))
      (Default|CallHackStarted)
      (EventDispatchers|AssignHackFinished (Variables|/Game/RebelX_Core/Blueprints/GM_RebelX.GM_RebelX_C|GetWidget _output_get) (delegate Custom|HackFinished_Event)))))

(fn ConstructionScript)

(fn GetAmmoInfo
  (return false "NewEnumerator0"))

(fn GetCrosshairPrompt
  (return (Variables|Default|GetPrompt) (Variables|Default|GetTooltip)))

(fn GetHealthInfo
  (return false 0.0))

(fn GetInteractionType
  (return false "NewEnumerator2"))

(fn GetIsConsumeable
  (return false))

(fn GetSceneInfo
  (return false))