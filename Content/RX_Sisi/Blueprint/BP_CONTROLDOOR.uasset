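; BP_CONTROLDOOR is an interactable door that slides open and offers an "OPEN DOOR" crosshair prompt.
; The Opendoor event plays a timeline that lerps the Door component from its current relative location toward a fixed offset, so motion compounds each update.
; Interaction getters supply the prompt and type and report no health, ammo or scene info.
; ActivateSceneObject is empty, and the file has no closing logic.
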(event Custom|Opendoor
  (bind _door (Variables|Default|Getdoor))
  (bind _新建轨道_0 (Timeline|时间轴 Play)
    (:Update
      (Transformation|SetRelativeLocation _door (Math|Vector|Lerp(Vector) (Variables|/Script/Engine.SceneComponent|GetRelativeLocation _door) "260.000000,0.000000,-20.000000" _新建轨道_0) false false))))

(event EventBeginPlay)

(event Collision|EventActorBeginOverlap
  (params (OtherActor :type Actor%20Object%20Reference)))

(event EventTick
  (params (DeltaSeconds :type Float%20%28single-precision%29)))

(event EventActivateSceneObject)

(fn ConstructionScript)

(fn GetCrosshairPrompt
  (return "OPEN DOOR" "[E] INTERACT"))

(fn GetIsConsumeable
  (return false))

(fn GetInteractionType
  (return false "NewEnumerator4"))

(fn GetHealthInfo
  (return false 0.0))

(fn GetAmmoInfo
  (return false "NewEnumerator0"))

(fn GetSceneInfo
  (return false))