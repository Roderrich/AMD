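; BP_DOOR is an interactable door that shows an "OPEN DOOR" crosshair prompt and opens when activated as a scene object.
; Its interaction getters mark it non-consumable and report no health, ammo or scene info.
; ActivateSceneObject calls OpenDoor, whose timeline slides one door mesh toward a fixed relative position.
; The lerp starts from the mesh's current location each update, so movement compounds; there is no closing logic.
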(event Custom|OpenDoor
  (bind _sm_bld_door_double_03_door_02 (Variables|Default|GetSM_Bld_Door_Double_03_Door_02))
  (bind _新建轨道_0 (Timeline|时间轴 PlayFromStart)
    (:Update
      (Transformation|SetRelativeLocation _sm_bld_door_double_03_door_02 (Math|Vector|Lerp(Vector) (Variables|/Script/Engine.SceneComponent|GetRelativeLocation _sm_bld_door_double_03_door_02) "260.000000,0.000000,-20.000000" _新建轨道_0) false false))))

(event EventBeginPlay)

(event Collision|EventActorBeginOverlap
  (params (OtherActor :type Actor%20Object%20Reference)))

(event EventTick
  (params (DeltaSeconds :type Float%20%28single-precision%29)))

(event EventActivateSceneObject
  (CallFunction|OpenDoor))

(fn ConstructionScript)

(fn GetCrosshairPrompt
  (return "OPEN DOOR" "[E] INTERACT"))

(fn GetIsConsumeable
  (return false))

(fn GetInteractionType
  (return false "NewEnumerator2"))

(fn GetHealthInfo
  (return false 0.0))

(fn GetAmmoInfo
  (return false "NewEnumerator0"))

(fn GetSceneInfo
  (return false))